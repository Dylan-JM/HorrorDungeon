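; BP_GlovesObject describes a glove item in the modular armor character clothing system.
; It supplies the mesh from its GlovesInfo data, and the glove type decides which body slot and morph targets it reports.
; All types except one target the hands body slot, and only one type reports the Gloves morph target.
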(fn `GetBodySlotsTargets`
  (returns (`Return Value` :type "Array of Name"))
  (if (`|EnumInequality` (`.GlovesType_5_3C2F12394B1D440C282491BFF6BD98BA` (break `/Game/ROG_Modular_Armor/Accessories_Robes/Blueprints/Utility/SROG_Accessories_Gloves` (`self.GlovesInfo`))) "NewEnumerator2")
    (return (`|MakeArray` "BODY_HANDS" :!type "Name"))))

(fn `GetMesh`
  (returns (`Return Value` :type "SkeletalMesh Object Reference"))
  (return (`.GlovesMesh_2_FF8FE721454E93DB5E4E02AB4CC1ADD4` (break `/Game/ROG_Modular_Armor/Accessories_Robes/Blueprints/Utility/SROG_Accessories_Gloves` (`self.GlovesInfo`)))))

(fn `GetMorphTargets`
  (returns (ReturnValue :type "Array of Name"))
  (if (`|EnumEquality` (`.GlovesType_5_3C2F12394B1D440C282491BFF6BD98BA` (break `/Game/ROG_Modular_Armor/Accessories_Robes/Blueprints/Utility/SROG_Accessories_Gloves` (`self.GlovesInfo`))) "NewEnumerator1")
    (return (`|MakeArray` "Gloves" :!type "Name"))))