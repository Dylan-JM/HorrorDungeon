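; Blueprint function library that creates cloth objects for the modular armor system, with one constructor per slot from helmet and bracers to cloak and robe.
; Each function constructs the slot's object class under the supplied Outer, passes in that slot's info and returns the new object.
; Left and right bracers have separate classes, both fed through a shared Bracers property.
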(fn `ConstructBootsCloth`
  (params (Outer :type "Object Object Reference") (BootsInfo :type "/Game/ROG_Modular_Armor/Armor_Cloth/Blueprints/Utility/SROG_Armor_Boots Structure"))
  (returns (ReturnValue :type "/Game/ROG_Modular_Armor/Characters/Blueprints/Cloths/BP_BaseClothObject Object Reference"))
  (bind _returnvalue (`|GenericCreateObject` Outer "/Game/ROG_Modular_Armor/Characters/Blueprints/Cloths/ArmorObjects/BP_BaseBootsObject.BP_BaseBootsObject_C" BootsInfo))
  (return _returnvalue))

(fn `ConstructChestCloth`
  (params (Outer :type "Object Object Reference") (ChestInfo :type "/Game/ROG_Modular_Armor/Armor_Cloth/Blueprints/Utility/SROG_Armor_Chests Structure"))
  (returns (ReturnValue :type "/Game/ROG_Modular_Armor/Characters/Blueprints/Cloths/BP_BaseClothObject Object Reference"))
  (bind _returnvalue (`|GenericCreateObject` Outer "/Game/ROG_Modular_Armor/Characters/Blueprints/Cloths/ArmorObjects/BP_BaseChestObject.BP_BaseChestObject_C" ChestInfo))
  (return _returnvalue))

(fn `ConstructCloakCloth`
  (params (Outer :type "Object Object Reference") (CloakInfo :type "/Game/ROG_Modular_Armor/Accessories_Robes/Blueprints/Utility/SROG_Accessories_Cloaks Structure"))
  (returns (ReturnValue :type "/Game/ROG_Modular_Armor/Characters/Blueprints/Cloths/BP_BaseClothObject Object Reference"))
  (bind _returnvalue (`|GenericCreateObject` Outer "/Game/ROG_Modular_Armor/Characters/Blueprints/Cloths/AccessoriesObjects/BP_CloakObject.BP_CloakObject_C" CloakInfo))
  (return _returnvalue))

(fn `ConstructGlovesCloth`
  (params (Outer :type "Object Object Reference") (GlovesInfo :type "/Game/ROG_Modular_Armor/Accessories_Robes/Blueprints/Utility/SROG_Accessories_Gloves Structure"))
  (returns (ReturnValue :type "/Game/ROG_Modular_Armor/Characters/Blueprints/Cloths/BP_BaseClothObject Object Reference"))
  (bind _returnvalue (`|GenericCreateObject` Outer "/Game/ROG_Modular_Armor/Characters/Blueprints/Cloths/AccessoriesObjects/BP_GlovesObject.BP_GlovesObject_C" GlovesInfo))
  (return _returnvalue))

(fn `ConstructHelmetCloth`
  (params (Outer :type "Object Object Reference") (HelmetInfo :type "/Game/ROG_Modular_Armor/Armor_Cloth/Blueprints/Utility/SROG_Armor_Helmets Structure"))
  (returns (ReturnValue :type "/Game/ROG_Modular_Armor/Characters/Blueprints/Cloths/BP_BaseClothObject Object Reference"))
  (bind _returnvalue (`|GenericCreateObject` Outer "/Game/ROG_Modular_Armor/Characters/Blueprints/Cloths/ArmorObjects/BP_BaseHelmetObject.BP_BaseHelmetObject_C" HelmetInfo))
  (return _returnvalue))

(fn `ConstructLeftBracersCloth`
  (params (Outer :type "Object Object Reference") (BracersInfo :type "/Game/ROG_Modular_Armor/Accessories_Robes/Blueprints/Utility/SROG_Accessories_Bracers Structure"))
  (returns (ReturnValue :type "/Game/ROG_Modular_Armor/Characters/Blueprints/Cloths/BP_BaseClothObject Object Reference"))
  (bind _returnvalue (`|GenericCreateObject` Outer "/Game/ROG_Modular_Armor/Characters/Blueprints/Cloths/AccessoriesObjects/BP_LeftBracerObject.BP_LeftBracerObject_C" BracersInfo))
  (return _returnvalue))

(fn `ConstructPantsCloth`
  (params (Outer :type "Object Object Reference") (PantsInfo :type "/Game/ROG_Modular_Armor/Armor_Cloth/Blueprints/Utility/SROG_Armor_Pants Structure"))
  (returns (ReturnValue :type "/Game/ROG_Modular_Armor/Characters/Blueprints/Cloths/BP_BaseClothObject Object Reference"))
  (bind _returnvalue (`|GenericCreateObject` Outer "/Game/ROG_Modular_Armor/Characters/Blueprints/Cloths/ArmorObjects/BP_BasePantsObject.BP_BasePantsObject_C" PantsInfo))
  (return _returnvalue))

(fn `ConstructRightBracerCloth`
  (params (Outer :type "Object Object Reference") (BracerInfo :type "/Game/ROG_Modular_Armor/Accessories_Robes/Blueprints/Utility/SROG_Accessories_Bracers Structure"))
  (returns (ReturnValue :type "/Game/ROG_Modular_Armor/Characters/Blueprints/Cloths/BP_BaseClothObject Object Reference"))
  (bind _returnvalue (`|GenericCreateObject` Outer "/Game/ROG_Modular_Armor/Characters/Blueprints/Cloths/AccessoriesObjects/BP_RightBracerObject.BP_RightBracerObject_C" BracerInfo))
  (return _returnvalue))

(fn `ConstructRobeCloth`
  (params (Outer :type "Object Object Reference") (RobeInfo :type "/Game/ROG_Modular_Armor/Accessories_Robes/Blueprints/Utility/SROG_Accessories_Robes Structure"))
  (returns (ReturnValue :type "/Game/ROG_Modular_Armor/Characters/Blueprints/Cloths/BP_BaseClothObject Object Reference"))
  (bind _returnvalue (`|GenericCreateObject` Outer "/Game/ROG_Modular_Armor/Characters/Blueprints/Cloths/AccessoriesObjects/BP_RobeObject.BP_RobeObject_C" RobeInfo))
  (return _returnvalue))

(fn `ConstructShouldersCloth`
  (params (Outer :type "Object Object Reference") (ShouldersInfo :type "/Game/ROG_Modular_Armor/Accessories_Robes/Blueprints/Utility/SROG_Accessories_Shoulders Structure"))
  (returns (ReturnValue :type "/Game/ROG_Modular_Armor/Characters/Blueprints/Cloths/BP_BaseClothObject Object Reference"))
  (bind _returnvalue (`|GenericCreateObject` Outer "/Game/ROG_Modular_Armor/Characters/Blueprints/Cloths/AccessoriesObjects/BP_ShouldersObject.BP_ShouldersObject_C" ShouldersInfo))
  (return _returnvalue))