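; BP_BasePantsObject is the base armor object for pants in the modular armor system.
; It supplies the mesh from its PantsInfo data and targets the legs body slot.
; It also defines the range for the "fatbody" morph target, bounded to a narrow span just above zero.
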(fn `GetBodySlotsTargets`
  (returns (`Return Value` :type "Array of Name"))
  (return (`|MakeArray` "BODY_LEGS" :!type "Name")))

(fn `GetMesh`
  (returns (`Return Value` :type "SkeletalMesh Object Reference"))
  (return (`.PantsMesh_2_1A569A324AC8DD3DBA02609741EF9E73` (break `/Game/ROG_Modular_Armor/Armor_Cloth/Blueprints/Utility/SROG_Armor_Pants` (`self.PantsInfo`)))))

(fn `GetMorphTargetsRange`
  (returns (`Return Value` :type "Map of Name to FloatRange Structure"))
  (return (`|MakeMap` "fatbody" (make `FloatRange` (make `FloatRangeBound` "Open") (make `FloatRangeBound` "Open" 0.15)) :!type "Name")))