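; BP_BaseChestObject is the base chest piece object in the modular armor system, supplying its mesh and the body slots it targets.
; GetMesh returns the chest mesh from the ChestInfo data.
; GetBodySlotsTargets builds a list of slot names from the same data, adding BODY_CHEST for one chest type and BODY_ARMS for one sleeve type.
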(fn `GetBodySlotsTargets`
  (returns (`Return Value` :type "Array of Name"))
  (locals (_Targets :type "Array of Name"))
  (bind (_chestmesh _chesttype _sleevetype) (break `/Game/ROG_Modular_Armor/Armor_Cloth/Blueprints/Utility/SROG_Armor_Chests` (`self.ChestInfo`)))
  (`|ExecutionSequence`
    (:`then_0`
      (if (`|EnumEquality` _chesttype "NewEnumerator0")
        (`KismetArrayLibrary.Array_Add` (`local._Targets`) "BODY_CHEST")))
    (:`then_1`
      (if (`|EnumEquality` _sleevetype "NewEnumerator1")
        (`KismetArrayLibrary.Array_Add` (`local._Targets`) "BODY_ARMS")))
    (:`then_2`
      (return (`local._Targets`)))))

(fn `GetMesh`
  (returns (`Return Value` :type "SkeletalMesh Object Reference"))
  (return (`.ChestMesh_2_44346292442DC3579C405987C0B22ED3` (break `/Game/ROG_Modular_Armor/Armor_Cloth/Blueprints/Utility/SROG_Armor_Chests` (`self.ChestInfo`)))))