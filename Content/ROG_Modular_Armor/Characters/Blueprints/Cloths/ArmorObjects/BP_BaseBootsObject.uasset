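; BP_BaseBootsObject is the base armor object for boots in the modular armor system, driven by a BootsInfo struct.
; It supplies the boot mesh and picks a low, high or empty morph target from the boot height.
; It reports the feet body slot as a target only for one boot type, and never for slippers.
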(fn `GetBodySlotsTargets`
  (returns (`Return Value` :type "Array of Name"))
  (bind ((`Type_8_55973A5741EC4889111533B96E806547` _type) (`Height_10_3F05CFB745ADBD6FE9EEB6A9D16CAA0E` _height)) (break `/Game/ROG_Modular_Armor/Armor_Cloth/Blueprints/Utility/SROG_Armor_Boots` (`self.BootsInfo`)))
  (if (and (`|EnumEquality` _type "NewEnumerator1") (`|EnumInequality` _height "NewEnumerator2"))
    (return (`|MakeArray` "BODY_FEET" :!type "Name"))))

(fn `GetMesh`
  (returns (`Return Value` :type "SkeletalMesh Object Reference"))
  (return (`.Mesh_7_406F0BE5460ECE429935D69BE0B51307` (break `/Game/ROG_Modular_Armor/Armor_Cloth/Blueprints/Utility/SROG_Armor_Boots` (`self.BootsInfo`)))))

(fn `GetMorphTargets`
  (returns (ReturnValue :type "Array of Name"))
  (locals (_Target :type "Array of Name"))
  (return (`|MakeArray` (select `/Game/ROG_Modular_Armor/Armor_Cloth/Blueprints/Utility/EROG_Boots_Height` (`.Height_10_3F05CFB745ADBD6FE9EEB6A9D16CAA0E` (break `/Game/ROG_Modular_Armor/Armor_Cloth/Blueprints/Utility/SROG_Armor_Boots` (`self.BootsInfo`))) :`NewEnumerator0` "Boots_low" :`NewEnumerator1` "Boots_high" :!type "Name"))))