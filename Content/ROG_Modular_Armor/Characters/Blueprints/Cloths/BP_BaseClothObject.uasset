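; Base cloth object for modular armor that applies and removes a clothing piece on its owning outer object.
; Getters supply the mesh, owner mesh tag, morph targets, morph ranges and body slots, with most left empty as hooks for subclasses.
; Add and remove functions send these to the outer object through interface-style messages, with removal clearing the tagged mesh and undoing morph and slot changes.
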(fn `AddBodySlotsTargets`
  (if (> (`KismetArrayLibrary.Array_Length` (`self.GetBodySlotsTargets`)) 0)
    (message `/Game/ROG_Modular_Armor/Characters/Blueprints/Cloths/BPI_ClothInterface.AddBodySlotsTargets` (`KismetSystemLibrary.GetOuterObject` self) (`self.GetBodySlotsTargets`))))

(fn `AddClothToOwner`
  (message `/Game/ROG_Modular_Armor/Characters/Blueprints/Cloths/BPI_ClothInterface.SetClothMeshByTag` (`KismetSystemLibrary.GetOuterObject` self) (`self.GetMesh`) (`self.GetMeshTagOnOwner`))
  (`self.AddMorphTargetsRange`)
  (`self.AddMorpthTargets`)
  (`self.AddBodySlotsTargets`))

(fn `AddMorphTargetsRange`
  (locals (_Keys :type "Array of Name") (_Values :type "Array of FloatRange Structure"))
  (bind _keys (`BlueprintMapLibrary.Map_Keys` (`self.GetMorphTargetsRange`)))
  (set `local._Keys` _keys)
  (bind _values (`BlueprintMapLibrary.Map_Values` (`self.GetMorphTargetsRange`)))
  (set `local._Values` _values)
  (for (_array_element _array_index) (`local._Keys`)
    (message `/Game/ROG_Modular_Armor/Characters/Blueprints/Cloths/BPI_ClothInterface.AddMorphTargetRange` (`KismetSystemLibrary.GetOuterObject` self) _array_element (`|GetArrayItem` (`local._Values`) _array_index))))

(fn `AddMorpthTargets`
  (for _array_element (`self.GetMorphTargets`)
    (message `/Game/ROG_Modular_Armor/Characters/Blueprints/Cloths/BPI_ClothInterface.AddMorphTarget` (`KismetSystemLibrary.GetOuterObject` self) _array_element)))

(fn `GetBodySlotsTargets`
  (returns (`Return Value` :type "Array of Name"))
  (return))

(fn `GetMesh`
  (returns (`Return Value` :type "SkeletalMesh Object Reference"))
  (return null))

(fn `GetMeshTagOnOwner`
  (returns (`Return Value` :type Name))
  (return (`self.ClothTagOnOwner`)))

(fn `GetMorphTargets`
  (returns (ReturnValue :type "Array of Name"))
  (return))

(fn `GetMorphTargetsRange`
  (returns (`Return Value` :type "Map of Name to FloatRange Structure"))
  (return))

(fn `GetType`
  (returns (`Return Value` :type "/Game/ROG_Modular_Armor/Characters/Blueprints/EClothType Enum"))
  (return (`self.ClothType`)))

(fn `RemoveBodySlotsTargets`
  (if (> (`KismetArrayLibrary.Array_Length` (`self.GetBodySlotsTargets`)) 0)
    (message `/Game/ROG_Modular_Armor/Characters/Blueprints/Cloths/BPI_ClothInterface.RemoveBodySlotsTargets` (`KismetSystemLibrary.GetOuterObject` self) (`self.GetBodySlotsTargets`))))

(fn `RemoveClothFromOwner`
  (message `/Game/ROG_Modular_Armor/Characters/Blueprints/Cloths/BPI_ClothInterface.SetClothMeshByTag` (`KismetSystemLibrary.GetOuterObject` self) null (`self.GetMeshTagOnOwner`))
  (`self.RemoveMorphTargetsRange`)
  (`self.RemoveMorphTargets`)
  (`self.RemoveBodySlotsTargets`))

(fn `RemoveMorphTargets`
  (for _array_element (`self.GetMorphTargets`)
    (message `/Game/ROG_Modular_Armor/Characters/Blueprints/Cloths/BPI_ClothInterface.RemoveMorphTarget` (`KismetSystemLibrary.GetOuterObject` self) _array_element)))

(fn `RemoveMorphTargetsRange`
  (locals (_Keys :type "Array of Name"))
  (bind _keys (`BlueprintMapLibrary.Map_Keys` (`self.GetMorphTargetsRange`)))
  (bind _output_get (set `local._Keys` _keys))
  (for _array_element _output_get
    (message `/Game/ROG_Modular_Armor/Characters/Blueprints/Cloths/BPI_ClothInterface.RemoveMorphTargetRange` (`KismetSystemLibrary.GetOuterObject` self) _array_element)))