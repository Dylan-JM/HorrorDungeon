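; Player character Blueprint for HorrorDungeon that links to its inventory component and manages starting equipment, item drops and turn animations.
; On a locally controlled restart, it equips starting weapon, armor and amulet classes through their default item objects.
; Loading a save rebuilds inventory items and replaces starting slots with saved equipment before re-equipping.
; Server events handle drops and multicast turn montages, while H toggles extreme global slow motion.
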(event `CombatInterface.SetInShockLoop`
  (params (InLoop :type Boolean))
  (set `self.InShockLoop` InLoop))

(event `CombatInterface.SetStartShock`
  (params (IsShock :type Boolean))
  (set `self.StartShock` IsShock))

(event `self.ReceiveBeginPlay`
  (`parent.ReceiveBeginPlay`)
  (bind _asbp_inventory_component_2 (cast `/Game/HorrorDungeon/Player/Components/BP_InventoryComponent2` (`self.InventoryComponent`)))
  (set `/Game/HorrorDungeon/Player/Components/BP_InventoryComponent2.PlayerCharacter` self _asbp_inventory_component_2))

(event `ServerPlayTurnAnimation`
  (params (MontageToPlay :type "AnimMontage Object Reference"))
  (`self.MulticastPlayTurnAnimation` MontageToPlay))

(event `self.EquipStartingItems`
  (`self.EquipStartingItemsBP`))

(event `MulticastPlayTurnAnimation`
  (params (MontageToPlay :type "AnimMontage Object Reference"))
  (`|PlayMontage` (`self.Mesh`) MontageToPlay
    (:`OnCompleted`
      _)
    (:`OnBlendOut`
      _)
    (:`OnInterrupted`
      _))
  (set `self.Turning` false))

(event `self.ReceiveRestarted`
  (if (`self.IsLocallyControlled`)
    (`KismetSystemLibrary.Delay` 0.2)
    (bind _asbp_inventory_component_2 (cast `/Game/HorrorDungeon/Player/Components/BP_InventoryComponent2` (`self.InventoryComponent`)))
    (set `self.BPInvComponent` _asbp_inventory_component_2)
    (`self.EquipStartingItemsBP`)))

(event `self.EmptyInventory`
  (`parent.EmptyInventory`)
  (`/Game/HorrorDungeon/Player/Components/BP_InventoryComponent2.EmptyInventory` (`self.BPInvComponent`)))

(event `self.AddSavedItemsToInventory`
  (bind _bpinvcomponent (`self.BPInvComponent`))
  (for _array_element (`LoadScreenSaveGame.SavedInventory` (`self.PlayerSaveGame`))
    (bind (_item _itemvalues) (break `SavedItems` _array_element))
    (bind _returnvalue (`|GenericCreateObject` "/Game/HorrorDungeon/Actor/UObject/BP_ItemObject.BP_ItemObject_C" (`.ItemObjectValues` (break `ItemValues` _itemvalues))))
    (if (`KismetSystemLibrary.IsValidClass` _item)
      (`/Game/HorrorDungeon/Player/Components/BP_InventoryComponent2.AddItemAt` _bpinvcomponent _returnvalue _itemvalues)
      (`InventoryComponent.AddItemToInventory` _bpinvcomponent (`.ItemValues` (break `SavedItems` _array_element)))))
  (`self.SetStartingItemsToNull`)
  (`self.SetStartingItems`)
  (`self.EquipStartingItemsBP`))

(event `Key|H`
  (params (Key :type "Key Structure"))
  (:`Pressed`
    (`/Engine/EditorBlueprintResources/StandardMacros.FlipFlop`
      (:`A`
        (`GameplayStatics.SetGlobalTimeDilation` 0.005))
      (:`B`
        (`GameplayStatics.SetGlobalTimeDilation` 1.0)))))

(event `ServerDropItem`
  (params (ActorToSpawn :type "EquippableActor Class Reference") (GroundClamp :type Boolean))
  (`self.SpawnItemFromActor` ActorToSpawn GroundClamp))

(fn `AddStartingItem`
  (params (ActorClass :type "EquippableActor Class Reference") (SlotNumber :type Integer))
  (bind _returnvalue (`GameplayStatics.GetActorOfClass` ActorClass))
  (bind _returnvalue_2 (`EquippableActor.GetDefaultItemObject` _returnvalue))
  (bind _asbp_item_object (cast `/Game/HorrorDungeon/Actor/UObject/BP_ItemObject` _returnvalue_2))
  (`/Game/HorrorDungeon/Player/Components/BP_InventoryComponent2.AddArmorWeapIfAvailable` (`self.BPInvComponent`) _asbp_item_object (`ItemObject.GetItemType` _asbp_item_object) (`local.SlotNumber`)))

(fn `EquipStartingItemsBP`
  (`|ExecutionSequence`
    (:`then_0`
      (bind _weapon1 (`self.Weapon1`)
        (:`then`
          (`self.AddStartingItem` _weapon1 1))
        (:`else`)))
    (:`then_1`
      (bind _offhanditem (`self.OffhandItem`)
        (:`then`
          (`self.AddStartingItem` _offhanditem 2))
        (:`else`)))
    (:`then_2`
      (bind _startinghelmet (`self.StartingHelmet`)
        (:`then`
          (`self.AddStartingItem` _startinghelmet))
        (:`else`)))
    (:`then_3`
      (bind _startingchestplate (`self.StartingChestplate`)
        (:`then`
          (`self.AddStartingItem` _startingchestplate))
        (:`else`)))
    (:`then_4`
      (bind _startinggauntlets (`self.StartingGauntlets`)
        (:`then`
          (`self.AddStartingItem` _startinggauntlets))
        (:`else`)))
    (:`then_5`
      (bind _startinglegs (`self.StartingLegs`)
        (:`then`
          (`self.AddStartingItem` _startinglegs))
        (:`else`)))
    (:`then_6`
      (bind _startingamulet1 (`self.StartingAmulet1`)
        (:`then`
          (`self.AddStartingItem` _startingamulet1 1))
        (:`else`)))
    (:`then_7`
      (bind _startingamulet2 (`self.StartingAmulet2`)
        (:`then`
          (`self.AddStartingItem` _startingamulet2 2))
        (:`else`)))
    (:`then_8`
      (bind _startingamulet3 (`self.StartingAmulet3`)
        (:`then`
          (`self.AddStartingItem` _startingamulet3 3))
        (:`else`)))))

(fn `SetStartingItems`
  (bind _playersavegame (`self.PlayerSaveGame`))
  (`|ExecutionSequence`
    (:`then_0`
      (set `self.Weapon1` (`LoadScreenSaveGame.EquippedWeapon1` _playersavegame)))
    (:`then_1`
      (set `self.OffhandItem` (`LoadScreenSaveGame.EquippedOffHandItem` _playersavegame)))
    (:`then_2`
      (set `self.StartingHelmet` (`LoadScreenSaveGame.EquippedHelmet` _playersavegame)))
    (:`then_3`
      (set `self.StartingChestplate` (`LoadScreenSaveGame.EquippedChestplate` _playersavegame)))
    (:`then_4`
      (set `self.StartingGauntlets` (`LoadScreenSaveGame.EquippedGaunlets` _playersavegame)))
    (:`then_5`
      (set `self.StartingLegs` (`LoadScreenSaveGame.EquippedLegs` _playersavegame)))
    (:`then_6`
      (set `self.StartingAmulet1` (`LoadScreenSaveGame.EquippedAmulet1` _playersavegame)))
    (:`then_7`
      (set `self.StartingAmulet2` (`LoadScreenSaveGame.EquippedAmulet2` _playersavegame)))
    (:`then_8`
      (set `self.StartingAmulet3` (`LoadScreenSaveGame.EquippedAmulet3` _playersavegame)))))

(fn `SetStartingItemsToNull`
  (`|ExecutionSequence`
    (:`then_0`
      (set `self.StartingHelmet` null))
    (:`then_1`
      (set `self.StartingChestplate` null))
    (:`then_2`
      (set `self.StartingLegs` null))
    (:`then_3`
      (set `self.StartingGauntlets` null))
    (:`then_4`
      (set `self.Weapon1` null))
    (:`then_5`
      (set `self.OffhandItem` null))
    (:`then_6`
      (set `self.StartingAmulet1` null))
    (:`then_7`
      (set `self.StartingAmulet2` null))
    (:`then_8`
      (set `self.StartingAmulet3` null))))

(fn `UserConstructionScript`)