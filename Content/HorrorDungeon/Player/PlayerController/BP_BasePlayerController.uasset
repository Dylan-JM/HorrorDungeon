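; Base player controller for the horror dungeon game that caches the possessed player character and handles picking up ground items into its inventory.
; Pickups first top up a matching unfilled stack, otherwise they go through the inventory component as a new item.
; A newly added arrow item shows the equipped bow's arrow mesh via local and server calls, activating fire if enabled.
; Collected actors have their type-specific visuals switched off before destruction.
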(event `self.ReceivePossess`
  (params (PossessedPawn :type "Pawn Object Reference"))
  (bind _asbp_player_character (cast `/Game/HorrorDungeon/Player/Characters/BP_PlayerCharacter` PossessedPawn))
  (set `self.BPPlayerCharacter` _asbp_player_character))

(event `ServerSetArrowVisibility`
  (params (NewVisibility :type Boolean) (Bow :type "Bow Object Reference"))
  (`SceneComponent.SetVisibility` (`Bow.ArrowMesh` Bow) NewVisibility false))

(event `self.AddItemToInventory`
  (bind _equippableactor (`self.EquippableActor`))
  (bind _returnvalue (`EquippableActor.GetDefaultItemObject` _equippableactor))
  (if (`EquippableActor.bOnGround` _equippableactor)
    (bind (_icon _iconrotated _itemclass _dimensions _itemtype _brotated _bistwohanded _maxstacks) (break `ItemObjectValues` (`ItemObject.ItemObjectValues` _returnvalue)))
    (if (> _maxstacks 1)
      (for _array_element (`/Game/HorrorDungeon/Player/Components/BP_InventoryComponent2.ItemsBP` (`/Game/HorrorDungeon/Player/Characters/BP_PlayerCharacter.BPInvComponent` (`self.BPPlayerCharacter`)))
        (`/Engine/EditorBlueprintResources/StandardMacros.IsValid` _array_element
          (:`Is Valid`
            (bind (_icon_2 _iconrotated_2 _itemclass_2 _dimensions_2 _itemtype_2 _brotated_2 _bistwohanded_2 _maxstacks_2 _currentstacks) (break `ItemObjectValues` (`ItemObject.ItemObjectValues` _array_element)))
            (if (== _itemclass_2 _itemclass)
              (if (not (== _maxstacks_2 _currentstacks))
                (set `self.bArrowFound` true)
                (set `ItemObject.ItemObjectValues` (make `ItemObjectValues` _icon_2 _iconrotated_2 _itemclass_2 _dimensions_2 _itemtype_2 _brotated_2 _bistwohanded_2 _maxstacks_2 (+ _currentstacks 1)) _array_element)
                (break))))))
      (if (`self.bArrowFound`)
        (set `self.bArrowFound` false)
        (set `EquippableActor.bOnGround` false (`self.EquippableActor`))
        (`self.ClientDestroyActor`)
        (`/Game/HorrorDungeon/Player/Components/BP_InventoryComponent2.OnInventoryChanged` (`/Game/HorrorDungeon/Player/Characters/BP_PlayerCharacter.BPInvComponent` (`self.BPPlayerCharacter`)))
        (else
          (bind (_added _itemvalues) (`/Game/HorrorDungeon/Player/Components/BP_InventoryComponent2.TryAddItem` (`/Game/HorrorDungeon/Player/Characters/BP_PlayerCharacter.BPInvComponent` (`self.BPPlayerCharacter`)) _returnvalue :!label _label))
          (if _added
            (`InventoryComponent.AddItemToInventory` (`BaseCharacter.InventoryComponent` (`self.BPPlayerCharacter`)) _itemvalues)
            (set `EquippableActor.bOnGround` false (`self.EquippableActor`))
            (if (== (`.ItemClass` (break `ItemObjectValues` (`ItemObject.ItemObjectValues` (`EquippableActor.ItemObject` (`self.EquippableActor`))))) "/Game/HorrorDungeon/Actor/Weapons/Bow/BP_InventoryArrow.BP_InventoryArrow_C")
              (bind _asbow (cast `Bow` (`BaseCharacter.EquippedWeapon1` (`self.BPPlayerCharacter`)))
                (:`then`
                  (bind _output_get (set `self.Bow` _asbow))
                  (`SceneComponent.SetVisibility` (`Bow.ArrowMesh` _output_get) true false)
                  (`self.ServerSetArrowVisibility` true (`self.Bow`))
                  (if (`BaseCharacter.bUseFireArrow` (`self.BPPlayerCharacter`))
                    (`ActorComponent.Activate` (`Bow.FireComponent` (`self.Bow`)) false))
                  (`self.ClientDestroyActor`))
                (:`CastFailed`
                  (`self.ClientDestroyActor`)))
              (else
                (`self.ClientDestroyActor`))))))
      (else
        (goto _label)))))

(event `ClientDestroyActor`
  (bind _equippableactor (`self.EquippableActor`)
    (:`then`
      (`SceneComponent.SetVisibility` (`EquippableActor.ItemMesh` _equippableactor) false false)
      (bind _asarmor (cast `Armor` (`self.EquippableActor`))
        (:`then`
          (`SceneComponent.SetVisibility` (`Armor.ArmorMeshComponent` _asarmor) false false))
        (:`CastFailed`
          (bind _ashand_held_torch (cast `HandHeldTorch` (`self.EquippableActor`))
            (:`then`
              (`HandHeldTorch.ToggleLight` _ashand_held_torch false))
            (:`CastFailed`
              (bind _asbow (cast `Bow` (`self.EquippableActor`))
                (:`then`
                  (`SceneComponent.SetVisibility` (`Bow.BowMeshComponent` _asbow) false false))
                (:`CastFailed`
                  _))))))
      (`self.K2_DestroyActor`))
    (:`else`)))

(event `ServerDestroyActor`
  (`self.EquippableActor`
    (:`then`
      (`self.K2_DestroyActor`))
    (:`else`)))

(fn `UserConstructionScript`)