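; Grid inventory component for HorrorDungeon that stores multi-tile items and manages armor, weapon and amulet equipment slots.
; TryAddItem scans the flat tile array for room, retrying rotated, and AddItemAt fills each covered cell.
; Equipping returns the slot's previous item to the grid, blocks two-handed conflicts and calls EquipItem on the player character.
; Adds and removals set a dirty flag, so Tick fires one inventory-changed notification.
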(event `self.ReceiveBeginPlay`
  (`KismetArrayLibrary.Array_Resize` (`self.ItemsBP`) (* (`self.Columns`) (`self.Rows`))))

(event `ServerAddItemAt`
  (params (ItemObject :type "ItemObject Object Reference") (TopLeftIndex :type Integer))
  (`self.AddItemAt` ItemObject (make `ItemValues` TopLeftIndex)))

(event `self.ReceiveTick`
  (params (DeltaSeconds :type "Float (single-precision)"))
  (if (`self.IsDirty`)
    (set `self.IsDirty` false)
    (`self.OnInventoryChanged`)))

(fn `AddArmorWeapIfAvailable`
  (params (ItemObject :type "ItemObject Object Reference") (SlotType :type "EItemType Enum" :default "EIT_Helmet") (SlotNumber :type Integer))
  (returns (Added :type Boolean))
  (bind (_itemobjectvalues_icon _itemobjectvalues_iconrotated _itemobjectvalues_itemclass) (break `ItemObjectValues` (`ItemObject.ItemObjectValues` ItemObject)))
  (if (and (`|EnumEquality` SlotType "EIT_Weapon") (not (`KismetMathLibrary.ClassIsChildOf` _itemobjectvalues_itemclass "/Script/HorrorDungeon.BaseWeapon")) (== SlotNumber 1))
    (return false)
    (elif (`|EnumEquality` (`ItemObject.GetItemType` ItemObject) SlotType)
      (bind _added (`self.AddArmorWeapInSlot` (`local.ItemObject`) SlotNumber))
      (return _added)
      (else
        (return false)))))

(fn `AddArmorWeapInSlot`
  (params (ItemObject :type "ItemObject Object Reference") (SlotNumber :type Integer))
  (returns (Added :type Boolean))
  (bind _itemobject (`local.ItemObject`))
  (`/Engine/EditorBlueprintResources/StandardMacros.IsValid` _itemobject
    (:`Is Valid`
      (if (`Pawn.IsLocallyControlled` (`self.PlayerCharacter`))
        (switch `EItemType` (`ItemObject.GetItemType` _itemobject)
          (:`EIT_Helmet`
            (bind _helmetitemobject (`self.HelmetItemObject`)
              (:`then`
                (`self.TryAddItem` _helmetitemobject)
                (`PlayerCharacter.UnequipItem` (`self.PlayerCharacter`) "EIT_Helmet" 0))
              (:`else`
                _))
            (bind _output_get (set `self.HelmetItemObject` (`local.ItemObject`)))
            (`PlayerCharacter.EquipItem` (`self.PlayerCharacter`) (`ItemObject.GetItemClass` _output_get) (`ItemObject.GetItemType` (`local.ItemObject`)) 0)
            (return true))
          (:`EIT_Chest`
            (bind _chestitemobject (`self.ChestItemObject`)
              (:`then`
                (`self.TryAddItem` _chestitemobject)
                (`PlayerCharacter.UnequipItem` (`self.PlayerCharacter`) "EIT_Chest" 0))
              (:`else`
                _))
            (bind _output_get_2 (set `self.ChestItemObject` (`local.ItemObject`)))
            (`PlayerCharacter.EquipItem` (`self.PlayerCharacter`) (`ItemObject.GetItemClass` _output_get_2) (`ItemObject.GetItemType` (`local.ItemObject`)) 0)
            (return true))
          (:`EIT_Legs`
            (bind _legsitemobject (`self.LegsItemObject`)
              (:`then`
                (`self.TryAddItem` _legsitemobject)
                (`PlayerCharacter.UnequipItem` (`self.PlayerCharacter`) "EIT_Legs" 0))
              (:`else`
                _))
            (bind _output_get_3 (set `self.LegsItemObject` (`local.ItemObject`)))
            (`PlayerCharacter.EquipItem` (`self.PlayerCharacter`) (`ItemObject.GetItemClass` _output_get_3) (`ItemObject.GetItemType` (`local.ItemObject`)) 0)
            (return true))
          (:`EIT_Arms`
            (bind _armsitemobject (`self.ArmsItemObject`)
              (:`then`
                (`self.TryAddItem` _armsitemobject)
                (`PlayerCharacter.UnequipItem` (`self.PlayerCharacter`) "EIT_Arms" 0))
              (:`else`
                _))
            (bind _output_get_4 (set `self.ArmsItemObject` (`local.ItemObject`)))
            (`PlayerCharacter.EquipItem` (`self.PlayerCharacter`) (`ItemObject.GetItemClass` _output_get_4) (`ItemObject.GetItemType` (`local.ItemObject`)) 0)
            (return true))
          (:`EIT_Weapon`
            (switch `int` (`local.SlotNumber`)
              (:`1`
                (bind _offhanditemobject (`self.OffhandItemObject`)
                  (:`then`
                    (if (or (`.bIsTwoHanded` (break `ItemObjectValues` (`ItemObject.ItemObjectValues` _offhanditemobject))) (`.bIsTwoHanded` (break `ItemObjectValues` (`ItemObject.ItemObjectValues` (`local.ItemObject`)))))
                      (return false)
                      (else
                        _)))
                  (:`else`
                    _))
                (bind _weaponitemobject (`self.WeaponItemObject`)
                  (:`then`
                    (`self.TryAddItem` _weaponitemobject)
                    (`PlayerCharacter.UnequipItem` (`self.PlayerCharacter`) "EIT_Weapon" (`local.SlotNumber`)))
                  (:`else`
                    _))
                (bind _output_get_5 (set `self.WeaponItemObject` (`local.ItemObject`)))
                (`PlayerCharacter.EquipItem` (`self.PlayerCharacter`) (`ItemObject.GetItemClass` _output_get_5) (`ItemObject.GetItemType` (`local.ItemObject`)) (`local.SlotNumber`))
                (return true))
              (:`2`
                (bind _weaponitemobject_2 (`self.WeaponItemObject`)
                  (:`then`
                    (if (or (`.bIsTwoHanded` (break `ItemObjectValues` (`ItemObject.ItemObjectValues` _weaponitemobject_2))) (`.bIsTwoHanded` (break `ItemObjectValues` (`ItemObject.ItemObjectValues` (`local.ItemObject`)))))
                      (return false)
                      (else
                        _)))
                  (:`else`
                    _))
                (bind _offhanditemobject_2 (`self.OffhandItemObject`)
                  (:`then`
                    (`self.TryAddItem` _offhanditemobject_2)
                    (`PlayerCharacter.UnequipItem` (`self.PlayerCharacter`) "EIT_Weapon" (`local.SlotNumber`)))
                  (:`else`
                    _))
                (bind _output_get_6 (set `self.OffhandItemObject` (`local.ItemObject`)))
                (`PlayerCharacter.EquipItem` (`self.PlayerCharacter`) (`ItemObject.GetItemClass` _output_get_6) (`ItemObject.GetItemType` (`local.ItemObject`)) (`local.SlotNumber`))
                (return true))))
          (:`EIT_Amulet`
            (switch `int` (`local.SlotNumber`)
              (:`1`
                (bind _amulet1itemobject (`self.Amulet1ItemObject`)
                  (:`then`
                    (`self.TryAddItem` _amulet1itemobject)
                    (`PlayerCharacter.UnequipItem` (`self.PlayerCharacter`) "EIT_Amulet" (`local.SlotNumber`)))
                  (:`else`
                    _))
                (bind _output_get_7 (set `self.Amulet1ItemObject` (`local.ItemObject`)))
                (`PlayerCharacter.EquipItem` (`self.PlayerCharacter`) (`ItemObject.GetItemClass` _output_get_7) (`ItemObject.GetItemType` (`local.ItemObject`)) (`local.SlotNumber`))
                (return true))
              (:`2`
                (bind _amulet2itemobject (`self.Amulet2ItemObject`)
                  (:`then`
                    (`self.TryAddItem` _amulet2itemobject)
                    (`PlayerCharacter.UnequipItem` (`self.PlayerCharacter`) "EIT_Amulet" (`local.SlotNumber`)))
                  (:`else`
                    _))
                (bind _output_get_8 (set `self.Amulet2ItemObject` (`local.ItemObject`)))
                (`PlayerCharacter.EquipItem` (`self.PlayerCharacter`) (`ItemObject.GetItemClass` _output_get_8) (`ItemObject.GetItemType` (`local.ItemObject`)) (`local.SlotNumber`))
                (return true))
              (:`3`
                (bind _amulet3itemobject (`self.Amulet3ItemObject`)
                  (:`then`
                    (`self.TryAddItem` _amulet3itemobject)
                    (`PlayerCharacter.UnequipItem` (`self.PlayerCharacter`) "EIT_Amulet" (`local.SlotNumber`)))
                  (:`else`
                    _))
                (bind _output_get_9 (set `self.Amulet3ItemObject` (`local.ItemObject`)))
                (`PlayerCharacter.EquipItem` (`self.PlayerCharacter`) (`ItemObject.GetItemClass` _output_get_9) (`ItemObject.GetItemType` (`local.ItemObject`)) (`local.SlotNumber`))
                (return true)))))))))

(fn `AddItemAt`
  (params (ItemObject :type "ItemObject Object Reference") (ItemValues :type "ItemValues Structure"))
  (`/Engine/EditorBlueprintResources/StandardMacros.IsValid` ItemObject
    (:`Is Valid`
      (bind _tile (`self.ForEachIndex` ItemObject (`.TopLeftIndex` (break `ItemValues` ItemValues)))
        (:`LoopBody`
          (`KismetArrayLibrary.Array_Set` (`self.ItemsBP`) (`self.TileToIndex` _tile) (`local.ItemObject`)))
        (:`Completed`
          (set `self.IsDirty` true))))))

(fn `EmptyInventory`
  (bind _allitems (`self.GetAllItems`))
  (bind _keys (`BlueprintMapLibrary.Map_Keys` _allitems))
  (for _array_element _keys
    (`self.RemoveItem` _array_element)))

(fn `GetAllItems`
  (returns (AllItems :type "Map of ItemObject Object Reference to /Game/HorrorDungeon/Player/UI/Inventory/Tile Structure"))
  (locals (`AllItems (Local)` :type "Map of ItemObject Object Reference to /Game/HorrorDungeon/Player/UI/Inventory/Tile Structure") (`CurrentItemObject (Local)` :type "ItemObject Object Reference"))
  (for (_array_element _array_index) (`self.ItemsBP`)
    (bind _output_get (set `local.CurrentItemObject (Local)` _array_element))
    (`/Engine/EditorBlueprintResources/StandardMacros.IsValid` _output_get
      (:`Is Valid`
        (if (not (`BlueprintMapLibrary.Map_Contains` (`local.AllItems (Local)`) _array_element))
          (`BlueprintMapLibrary.Map_Add` (`local.AllItems (Local)`) (`local.CurrentItemObject (Local)`) (`self.IndexToTile` _array_index))))))
  (return (`local.AllItems (Local)`)))

(fn `GetItemAtIndex`
  (params (Index :type Integer))
  (returns (Valid :type Boolean) (ItemObject :type "ItemObject Object Reference"))
  (if (`KismetArrayLibrary.Array_IsValidIndex` (`self.ItemsBP`) Index)
    (return true (`|GetArrayItem` (`self.ItemsBP`) (`local.Index`)))
    (else
      (return false null))))

(fn `IndexToTile`
  (params (Index :type Integer))
  (returns (Tile :type "/Game/HorrorDungeon/Player/UI/Inventory/Tile Structure"))
  (return (make `/Game/HorrorDungeon/Player/UI/Inventory/Tile` (mod Index (`self.Columns`)) (/ Index (`self.Columns`)))))

(fn `IsRoomAvailable`
  (params (ItemObject :type "ItemObject Object Reference") (TopLeftIndex :type Integer))
  (returns (Result :type Boolean))
  (`|ExecutionSequence`
    (:`then_0`
      (bind _tile (`self.ForEachIndex` (`local.ItemObject`) (`local.TopLeftIndex`))
        (:`LoopBody`
          (`self.IsTileValid` _tile
            (:`true`
              (bind (_valid _itemobject) (`self.GetItemAtIndex` (`self.TileToIndex` _tile)))
              (if _valid
                (if (`KismetSystemLibrary.IsValid` _itemobject)
                  (return false))
                (else
                  (return false))))
            (:`false`
              (return false))))))
    (:`then_1`
      (return true))))

(fn `RemoveItem`
  (params (ItemObject :type "ItemObject Object Reference"))
  (bind _itemobject (`local.ItemObject`))
  (`/Engine/EditorBlueprintResources/StandardMacros.IsValid` ItemObject
    (:`Is Valid`
      (for (_array_element _array_index) (`self.ItemsBP`)
        (if (== _array_element _itemobject)
          (`KismetArrayLibrary.Array_Set` (`self.ItemsBP`) _array_index)
          (set `self.IsDirty` true)
          (`KismetArrayLibrary.Array_AddUnique` (`self.IndexArray`) _array_index)
          (bind _asbase_enemy (cast `BaseEnemy` (`self.GetOwner`)))
          (set `BaseEnemy.bHasItem` false _asbase_enemy)))
      (for _array_element_2 (`self.IndexArray`)
        (`BlueprintMapLibrary.Map_Remove` (`self.Inventory`) (make `ItemValues` _array_element_2 (`ItemObject.ItemObjectValues` _itemobject)))))))

(fn `TileToIndex`
  (params (Tile :type "/Game/HorrorDungeon/Player/UI/Inventory/Tile Structure"))
  (returns (Index :type Integer))
  (bind (_x _y) (break `/Game/HorrorDungeon/Player/UI/Inventory/Tile` Tile))
  (return (+ _x (* _y (`self.Columns`)))))

(fn `TryAddItem`
  (params (ItemObject :type "ItemObject Object Reference"))
  (returns (Added :type Boolean) (ItemValues :type "ItemValues Structure"))
  (bind _itemobject (`local.ItemObject`))
  (bind _itemobjectvalues (`ItemObject.ItemObjectValues` _itemobject))
  (`/Engine/EditorBlueprintResources/StandardMacros.IsValid` ItemObject
    (:`Is Valid`
      (set `/Game/HorrorDungeon/Actor/UObject/BP_ItemObject.Equipped` false ItemObject)
      (`/Engine/EditorBlueprintResources/StandardMacros.IsValid` ItemObject
        (:`Is Valid`
          (for (_ _array_index) (`self.ItemsBP`) :!label _label
            (bind _result (`self.IsRoomAvailable` (`local.ItemObject`) _array_index))
            (if _result
              (`self.AddItemAt` _itemobject (make `ItemValues` _array_index _itemobjectvalues))
              (return true (make `ItemValues` _array_index _itemobjectvalues))))
          (`|ExecutionSequence`
            (:`then_0`
              (`/Engine/EditorBlueprintResources/StandardMacros.DoOnce` false
                (:`Completed`
                  (`ItemObject.Rotate` (`local.ItemObject`))
                  (goto _label))))
            (:`then_1`
              (`ItemObject.Rotate` (`local.ItemObject`))
              (return false))))))))

(fn `Unequip`
  (params (ItemObject :type "ItemObject Object Reference") (SlotNumber :type Integer))
  (`/Engine/EditorBlueprintResources/StandardMacros.IsValid` ItemObject
    (:`Is Valid`
      (switch `EItemType` (`ItemObject.GetItemType` ItemObject)
        (:`EIT_Helmet`
          (set `self.HelmetItemObject` null))
        (:`EIT_Chest`
          (set `self.ChestItemObject` null))
        (:`EIT_Legs`
          (set `self.LegsItemObject` null))
        (:`EIT_Arms`
          (set `self.ArmsItemObject` null))
        (:`EIT_Weapon`
          (switch `int` (`local.SlotNumber`)
            (:`1`
              (set `self.WeaponItemObject` null))
            (:`2`
              (set `self.OffhandItemObject` null))))
        (:`EIT_Amulet`
          (switch `int` (`local.SlotNumber`)
            (:`1`
              (set `self.Amulet1ItemObject` null))
            (:`2`
              (set `self.Amulet2ItemObject` null))
            (:`3`
              (set `self.Amulet3ItemObject` null)))))
      (`PlayerCharacter.UnequipItem` (`self.PlayerCharacter`) (`ItemObject.GetItemType` (`local.ItemObject`)) (`local.SlotNumber`)))))

(fn `UnequipEquippedItems`
  (bind _chestplate (`BaseCharacter.Chestplate` (`self.PlayerCharacter`))
    (:`then`
      (`self.Unequip` (`EquippableActor.ItemObject` _chestplate)))
    (:`else`)))