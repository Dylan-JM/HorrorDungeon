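; GA_SelfRevive is a player support gameplay ability that lets a downed character revive themselves.
; If the owner is dead on the ground, it fires the revived callback, clears that state and applies the GE_ReviveHeal effect to itself.
; It then plays the revive montage, clearing the Dead flag and ending on any montage outcome; otherwise it ends immediately.
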(event `self.K2_ActivateAbility`
  (bind _ownercharacter (`self.OwnerCharacter`))
  (`self.StoreOwnerVariables`)
  (if (`BaseCharacter.bDeadOnGround` _ownercharacter)
    (`PlayerCharacter.OnPlayerRevived` _ownercharacter)
    (set `BaseCharacter.bDeadOnGround` false _ownercharacter)
    (`AbilitySystemComponent.BP_ApplyGameplayEffectToSelf` :`self` (`AbilitySystemBlueprintLibrary.GetAbilitySystemComponent` _ownercharacter) :`GameplayEffectClass` "/Game/HorrorDungeon/AbilitySystem/Player/Effects/Heals/GE_ReviveHeal.GE_ReviveHeal_C")
    (`AbilityTask_PlayMontageAndWait.CreatePlayMontageAndWaitProxy` "None" "/Game/Assets/Characters/Mannequins/MyAnimations/Montages/AM_Revive.AM_Revive"
      (:`OnCompleted`
        _)
      (:`OnBlendOut`
        _)
      (:`OnInterrupted`
        _)
      (:`OnCancelled`
        _))
    (set `BaseCharacter.bDead` false (`self.OwnerCharacter`))
    (`self.K2_EndAbility`)
    (else
      (`self.K2_EndAbility`))))