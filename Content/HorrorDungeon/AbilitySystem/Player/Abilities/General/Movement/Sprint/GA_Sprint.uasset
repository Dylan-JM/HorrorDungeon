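; GA_Sprint is the player's sprint Gameplay Ability, which refuses to run while aiming and otherwise forwards sprint press and release to the player controller.
; On activation it commits the ability, strips stamina regen effects and starts a looping timer that polls aiming and stamina.
; Input release, aiming or empty stamina stops sprinting, clears the timer and removes the sprint cost effect.
; After a short delay it reapplies GE_StaminaRegen and ends.
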(event `self.K2_ActivateAbility`
  (`self.StoreOwnerVariables`)
  (if (`BaseCharacter.bIsAiming` (`self.OwnerCharacter`))
    (`self.K2_EndAbility`)
    (else
      (`BasePlayerController.SprintButtonPressed` (`PlayerCharacter.PlayerCharacterController` (`self.OwnerCharacter`)))
      (`self.K2_CommitAbility`)
      (`self.BP_RemoveGameplayEffectFromOwnerWithAssetTags` (struct :`GameplayTags` (struct :`(TagName` "Effects.StaminaRegen"))))
      (bind _returnvalue (`KismetSystemLibrary.K2_SetTimerDelegate` (delegate `CheckStaminaAndAiming`) 0.1 true))
      (set `self.StaminaCheckTimer` _returnvalue)
      (`AbilityTask_WaitInputRelease.WaitInputRelease` false
        (:`OnRelease`
          (`BasePlayerController.SprintButtonReleased` (`PlayerCharacter.PlayerCharacterController` (`self.OwnerCharacter`)))
          (`self.PrepareEndAbility`)
          (`KismetSystemLibrary.Delay` 1.0)
          (`AbilitySystemComponent.BP_ApplyGameplayEffectToSelf` :`self` (`self.GetAbilitySystemComponentFromActorInfo`) :`GameplayEffectClass` "/Game/HorrorDungeon/AbilitySystem/Player/Effects/Heals/GE_StaminaRegen.GE_StaminaRegen_C")
          (`self.K2_EndAbility`))))))

(event `CheckStaminaAndAiming`
  (bind _ownercharacter (`self.OwnerCharacter`))
  (if (`BaseCharacter.bIsAiming` _ownercharacter)
    (`BasePlayerController.SprintButtonReleased` (`PlayerCharacter.PlayerCharacterController` (`self.OwnerCharacter`)) :!label _label)
    (`self.PrepareEndAbility`)
    (`KismetSystemLibrary.Delay` 1.5)
    (`AbilitySystemComponent.BP_ApplyGameplayEffectToSelf` :`self` (`self.GetAbilitySystemComponentFromActorInfo`) :`GameplayEffectClass` "/Game/HorrorDungeon/AbilitySystem/Player/Effects/Heals/GE_StaminaRegen.GE_StaminaRegen_C")
    (`self.K2_EndAbility`)
    (else
      (bind _returnvalue (`AbilitySystemComponent.GetAttributeSet` (`AbilitySystemBlueprintLibrary.GetAbilitySystemComponent` _ownercharacter) "/Script/HorrorDungeon.HDAttributeSet"))
      (bind _ashdattribute_set (cast `HDAttributeSet` _returnvalue))
      (if (== (`.CurrentValue` (break `GameplayAttributeData` (`HDAttributeSet.Stamina` _ashdattribute_set))) 0.0)
        (goto _label)))))

(fn `PrepareEndAbility`
  (`KismetSystemLibrary.K2_ClearAndInvalidateTimerHandle` (`self.StaminaCheckTimer`))
  (`self.BP_RemoveGameplayEffectFromOwnerWithGrantedTags` (struct :`GameplayTags` (struct :`(TagName` "Cost.Sprint")))))