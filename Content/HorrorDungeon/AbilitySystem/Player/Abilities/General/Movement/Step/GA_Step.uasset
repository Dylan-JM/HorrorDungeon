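; Player movement gameplay ability that performs a quick back or side step while the character is aiming and not falling.
; It rejects straight-forward input, removes the forward vector from forward diagonals, commits the cost, then launches the character along that vector.
; A back, left or right montage follows the movement direction, and its end generally clears the stepping state.
; Non-authority clients launch and animate locally, then use server events to replicate the step.
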(event `ClientStep`
  (bind _movementdirectionvector (`PlayerCharacter.MovementDirectionVector` (`self.OwnerCharacter`)))
  (bind (_x _y) (`KismetMathLibrary.BreakVector2D` _movementdirectionvector))
  (`self.PlayStepMontage` _movementdirectionvector)
  (if (== _y -1.0)
    ;[1 1 1] Is Back Stepping
    (`self.ServerPlayStepMontage` (`PlayerCharacter.MovementDirectionVector` (`self.OwnerCharacter`)))
    (`self.K2_EndAbility`)
    (else
      (`self.ServerLaunchCharacter` (`self.LastMovementInputVector`) null _x))))

(event `self.K2_ActivateAbility`
  (bind (_returnvalue_x _returnvalue_y) (`KismetMathLibrary.BreakVector` (* (`self.LastMovementInputVector`) 2000.0)))
  (`self.StoreOwnerVariables`)
  (if (`NavMovementComponent.IsFalling` (`Character.CharacterMovement` (`self.OwnerCharacter`)))
    (`self.K2_EndAbility` :!label _label)
    (elif (`BaseCharacter.bIsAiming` (`self.OwnerCharacter`))
      (message `CombatInterface.SetStepping` (`self.OwnerCharacter`) true)
      (bind _shouldstep (`self.SetLastMovementInputVector` (`self.OwnerCharacter`)))
      (if _shouldstep
        (bind _returnvalue (`self.K2_CommitAbilityCost` false))
        (if _returnvalue
          (`Character.LaunchCharacter` (`self.OwnerCharacter`) (`KismetMathLibrary.MakeVector` _returnvalue_x _returnvalue_y) false false)
          (if (`Actor.HasAuthority` (`self.OwnerCharacter`))
            (`self.PlayStepMontage` (`PlayerCharacter.MovementDirectionVector` (`self.OwnerCharacter`)))
            (else
              (`self.ClientStep`)))
          (else
            (message `CombatInterface.SetStepping` (`self.OwnerCharacter`) false)
            (`self.K2_EndAbility`)))
        (else
          (`self.K2_EndAbility`)))
      (else
        (goto _label)))))

(event `ServerPlayStepMontage`
  (params (MovementDirection :type "Vector2D Structure"))
  (`self.PlayStepMontage` MovementDirection))

(event `ServerLaunchCharacter`
  (params (LastMovementInputVector :type "Vector Structure") (CurrentCharacter :type "/Game/HorrorDungeon/Player/Characters/BP_PlayerCharacter Object Reference") (MovementDirectionVectorX :type "Float (double-precision)"))
  (bind (_returnvalue_x _returnvalue_y) (`KismetMathLibrary.BreakVector` (* LastMovementInputVector 2000.0)))
  (if (== MovementDirectionVectorX 0.0)
    (`self.K2_EndAbility`)
    (else
      (`Character.LaunchCharacter` CurrentCharacter (`KismetMathLibrary.MakeVector` _returnvalue_x _returnvalue_y) false false)
      (`self.PlayStepMontage` (`KismetMathLibrary.MakeVector2D` MovementDirectionVectorX)))))

(event `PlayStepMontage`
  (params (MovementDirectionVector :type "Vector2D Structure"))
  (if (== MovementDirectionVector_Y -1.0)
    (`AbilityTask_PlayMontageAndWait.CreatePlayMontageAndWaitProxy` "None" "/Game/Assets/Characters/Mannequins/MyAnimations/Montages/M_StepBack.M_StepBack" 1.0 "None" false
      (:`OnCompleted`
        _)
      (:`OnInterrupted`
        _)
      (:`OnCancelled`
        _))
    (message `CombatInterface.SetStepping` (`self.GetAvatarActorFromActorInfo`) false)
    (`self.K2_EndAbility`)
    (elif (== MovementDirectionVector_X 1.0)
      (`AbilityTask_PlayMontageAndWait.CreatePlayMontageAndWaitProxy` "None" "/Game/Assets/Characters/Mannequins/MyAnimations/Montages/AM_RightSideStep.AM_RightSideStep" 1.0 "None" false
        (:`OnCompleted`
          _)
        (:`OnInterrupted`
          _)
        (:`OnCancelled`
          _))
      (message `CombatInterface.SetStepping` (`self.GetAvatarActorFromActorInfo`) false)
      (`self.K2_EndAbility`)
      (elif (== MovementDirectionVector_X -1.0)
        (`AbilityTask_PlayMontageAndWait.CreatePlayMontageAndWaitProxy` "None" "/Game/Assets/Characters/Mannequins/MyAnimations/Montages/AM_LeftSideStep.AM_LeftSideStep" 1.0 "None" false
          (:`OnCompleted`
            (message `CombatInterface.SetStepping` (`self.GetAvatarActorFromActorInfo`) false)
            (`self.K2_EndAbility`)))
        (else
          (`self.K2_EndAbility`))))))

(fn `NewFunction`)

(fn `SetLastMovementInputVector`
  (params (PlayerCharacter :type "PlayerCharacter Object Reference"))
  (returns (ShouldStep :type Boolean))
  (bind _returnvalue (`Pawn.GetLastMovementInputVector` PlayerCharacter))
  (bind (_movementdirectionvector_x _movementdirectionvector_y) (`KismetMathLibrary.BreakVector2D` (`PlayerCharacter.MovementDirectionVector` PlayerCharacter)))
  (if (== _movementdirectionvector_y 1.0)
    (if (== _movementdirectionvector_x 0.0)
      (return false)
      (else
        (set `self.LastMovementInputVector` (- _returnvalue (`Actor.GetActorForwardVector` PlayerCharacter)))
        (return true)))
    (else
      (set `self.LastMovementInputVector` _returnvalue)
      (return true))))