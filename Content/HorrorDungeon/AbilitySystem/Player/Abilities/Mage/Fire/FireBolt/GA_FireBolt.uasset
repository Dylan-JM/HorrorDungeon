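; Mage Fire Bolt gameplay ability that casts a fire projectile when the owner holds a mage weapon, and ends immediately otherwise.
; It commits, flags the owner as attacking, and plays the fireball montage both directly and through a server event.
; A montage gameplay event triggers the projectile spawn, then turns the owner's capsule in yaw toward the hit target.
; Montage completion, blend-out or interruption clears the attacking flag and ends the ability.
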(event `self.K2_ActivateAbility`
  (bind (_returnvalue_roll _returnvalue_pitch _returnvalue_yaw) (`KismetMathLibrary.BreakRotator` (`KismetMathLibrary.FindLookAtRotation` (`SceneComponent.K2_GetComponentLocation` (`Character.CapsuleComponent` (`self.OwnerCharacter`))) (`self.HitTargetLoc`))))
  (`self.StoreOwnerVariables`)
  (bind _returnvalue (`self.IsCorrectWeapon` "/Script/HorrorDungeon.MageWeapon"))
  (if _returnvalue
    (`self.K2_CommitAbility`)
    (message `CombatInterface.SetIsAttacking` (`self.OwnerCharacter`) true)
    (`self.ServerPlayMontage`)
    (`AbilityTask_PlayMontageAndWait.CreatePlayMontageAndWaitProxy` "None" "/Game/Assets/Characters/Mannequins/MyAnimations/Montages/M_MG_Fireball_03.M_MG_Fireball_03" 1.0 "None" false
      (:`then`
        (`AbilityTask_WaitGameplayEvent.WaitGameplayEvent` (struct :`TagName` "Event.Montage.FireBolt") null
          (:`EventReceived`
            (`self.SpawnProjectiles` false 35.0)
            (`SceneComponent.K2_SetWorldRotation` (`Character.CapsuleComponent` (`self.OwnerCharacter`)) (`KismetMathLibrary.MakeRotator` 0.0 0.0 _returnvalue_yaw) false false))))
      (:`OnCompleted`
        (message `CombatInterface.SetIsAttacking` (`self.OwnerCharacter`) false :!label _label)
        (`self.K2_EndAbility`))
      (:`OnBlendOut`
        (goto _label))
      (:`OnInterrupted`
        (goto _label)))
    (else
      (`self.K2_EndAbility`))))

(event `ServerPlayMontage`
  (`AbilityTask_PlayMontageAndWait.CreatePlayMontageAndWaitProxy` "None" "/Game/Assets/Characters/Mannequins/MyAnimations/Montages/M_MG_Fireball_03.M_MG_Fireball_03" 1.0 "None" false))