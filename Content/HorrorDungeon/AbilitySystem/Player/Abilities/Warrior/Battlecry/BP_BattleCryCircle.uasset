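; BP_BattleCryCircle is the magic circle actor for the Warrior's Battlecry ability, shown briefly before the explosion.
; Tick slowly spins the circle decal around its local roll axis.
; One second after BeginPlay it spawns BP_BattleCryExplosion at its own location with the same owner, hands over its DamageEffectParams, then destroys itself.
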(event `self.ReceiveTick`
  (params (DeltaSeconds :type "Float (single-precision)"))
  (`SceneComponent.K2_AddLocalRotation` (`self.MagicCircleDecal`) (`KismetMathLibrary.MakeRotator` (* DeltaSeconds 8.0)) false false))

(event `self.ReceiveBeginPlay`
  (`KismetSystemLibrary.Delay` 1.0)
  (bind _returnvalue (`|SpawnActorFromClass` "/Game/HorrorDungeon/AbilitySystem/Player/Abilities/Warrior/Battlecry/BP_BattleCryExplosion.BP_BattleCryExplosion_C" (`KismetMathLibrary.MakeTransform` (`self.K2_GetActorLocation`)) "AdjustIfPossibleButAlwaysSpawn" "MultiplyWithRoot" (`self.GetOwner`) null))
  (bind _output_get (set `self.Explosion` _returnvalue))
  (set `HDProjectile.DamageEffectParams` (`self.DamageEffectParams`) _output_get)
  (`self.K2_DestroyActor`))

(fn `UserConstructionScript`)