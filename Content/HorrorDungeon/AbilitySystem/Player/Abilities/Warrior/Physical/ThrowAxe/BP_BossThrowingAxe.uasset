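; Thrown axe actor for a boss, which spins continuously once spawned and leaves any other behavior to its parent class.
; BeginPlay caches the RotationPoint's world roll and yaw, then a self-restarting timeline drives only its pitch.
; An unused helper, marked as probably unneeded, would destroy the axe with fire explosion sound and effects when its per-frame movement stalls.
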(event `SpinAxe`
  (bind (_direction _y_rotation) (`Timeline|RotationTimeline` :!via `PlayFromStart`)
    (:`Update`
      (`SceneComponent.K2_SetWorldRotation` (`self.RotationPoint`) (`KismetMathLibrary.MakeRotator` (`self.CurrentRotationValueX`) _y_rotation (`self.CurrentRotationValueZ`)) false false))
    (:`Finished`
      (`self.SpinAxe`))))

(event `self.ReceiveBeginPlay`
  (bind (_returnvalue_roll _returnvalue_pitch _returnvalue_yaw) (`KismetMathLibrary.BreakRotator` (`SceneComponent.K2_GetComponentRotation` (`self.RotationPoint`))))
  (`parent.ReceiveBeginPlay`)
  (set `self.CurrentRotationValueX` _returnvalue_roll)
  (set `self.CurrentRotationValueZ` _returnvalue_yaw)
  (`self.SpinAxe`))

(fn `MakeExplodeIfNoMove`
  (set `self.LocationLastFrame` (`self.LocationThisFrame`))
  (set `self.LocationThisFrame` (`self.K2_GetActorLocation`))
  (if (<= (`KismetMathLibrary.VSize` (- (`self.LocationThisFrame`) (`self.LocationLastFrame`))) (`self.MinDistancePerFrame`))
    (`GameplayStatics.SpawnSoundAtLocation` "/Game/Assets/Sounds/Abilities/FireBolt/sfx_FireBolt_Impact.sfx_FireBolt_Impact" (`self.LocationThisFrame`) (struct) 1.0 1.0 0.0 null null)
    (`NiagaraFunctionLibrary.SpawnSystemAtLocation` "/Game/Assets/Effects/Projectiles/FireExplosion/NS_FireExplosion.NS_FireExplosion" (`self.LocationThisFrame`))
    (`self.K2_DestroyActor`)))

(fn `UserConstructionScript`)