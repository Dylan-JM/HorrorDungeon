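; Short-lived explosion actor that sits with the Warrior's Radiant Strike ability assets.
; On BeginPlay it calls OnHit, whose body is not defined here, then destroys itself after a brief delay.
; An unused MakeExplodeIfNoMove, noted as probably unneeded, would spawn fire impact sound and Niagara effects and destroy the actor when its per-frame movement falls to a threshold.
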(event `self.ReceiveBeginPlay`
  (`self.OnHit`)
  (`KismetSystemLibrary.Delay` 1.0)
  (`self.K2_DestroyActor`))

(event `self.ReceiveTick`
  (params (DeltaSeconds :type "Float (single-precision)")))

(fn `MakeExplodeIfNoMove`
  (set `self.LocationLastFrame` (`self.LocationThisFrame`))
  (set `self.LocationThisFrame` (`self.K2_GetActorLocation`))
  (if (<= (`KismetMathLibrary.VSize` (- (`self.LocationThisFrame`) (`self.LocationLastFrame`))) (`self.MinDistancePerFrame`))
    (`GameplayStatics.SpawnSoundAtLocation` "/Game/Assets/Sounds/Abilities/FireBolt/sfx_FireBolt_Impact.sfx_FireBolt_Impact" (`self.LocationThisFrame`) (struct) 1.0 1.0 0.0 null null)
    (`NiagaraFunctionLibrary.SpawnSystemAtLocation` "/Game/Assets/Effects/Projectiles/FireExplosion/NS_FireExplosion.NS_FireExplosion" (`self.LocationThisFrame`))
    (`self.K2_DestroyActor`)))

(fn `UserConstructionScript`)