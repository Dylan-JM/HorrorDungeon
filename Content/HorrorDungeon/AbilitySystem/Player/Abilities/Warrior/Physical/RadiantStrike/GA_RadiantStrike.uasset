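; Warrior Radiant Strike gameplay ability: a montage-driven melee attack that ends in a line of radiant explosions along the weapon.
; After a melee weapon check, it sets damage, commits and plays the montage.
; Parallel montage event waits toggle the weapon's mesh swap and hit collision.
; The disable-collision event also spawns BP_RadiantExplosion actors evenly between blade Base and Tip sockets, each carrying radial physical damage, then ends the ability.
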(event `self.K2_ActivateAbility`
  (bind _returnvalue (`self.GetAvatarActorFromActorInfo`))
  (bind _itemmesh (`EquippableActor.ItemMesh` (`self.Melee Weapon`)))
  (`self.StoreOwnerVariables`)
  (bind _returnvalue_2 (`self.IsCorrectWeapon` "/Script/HorrorDungeon.MeleeWeapon"))
  (if _returnvalue_2
    (`self.SetDamage`)
    (bind _returnvalue_3 (message `CombatInterface.GetEquippedWeapon1` (`self.OwnerCharacter`)))
    (bind _asbp_melee_weapon (cast `/Game/HorrorDungeon/Actor/Weapons/Melee/BP_MeleeWeapon` _returnvalue_3))
    (set `self.Melee Weapon` _asbp_melee_weapon)
    (`self.K2_CommitAbility`)
    (`AbilityTask_PlayMontageAndWait.CreatePlayMontageAndWaitProxy` "None" "/Game/Assets/Characters/Mannequins/MyAnimations/Montages/AM_RadiantStrike.AM_RadiantStrike" 1.0 "None" false
      (:`then`
        (`AbilityTask_WaitGameplayEvent.WaitGameplayEvent` (struct :`TagName` "Montage.Attack.RadiantStrike") null
          (:`then`
            (`AbilityTask_WaitGameplayEvent.WaitGameplayEvent` (struct :`TagName` "Montage.Attack") null
              (:`then`
                (`AbilityTask_WaitGameplayEvent.WaitGameplayEvent` (struct :`TagName` "Montage.Attack.RadiantStrikeEnd") null
                  (:`then`
                    (`AbilityTask_WaitGameplayEvent.WaitGameplayEvent` (struct :`TagName` "Montage.Attack.DisableCollision") null
                      (:`EventReceived`
                        (`MeleeWeapon.AbilityHandleCollision` (`self.Melee Weapon`) false)
                        (for _array_element (`HDAbilitySystemLibrary.EvenlySpacedVectors` (`SceneComponent.GetSocketLocation` _itemmesh "Base") (`SceneComponent.GetSocketLocation` _itemmesh "Tip") 10.0 10)
                          (bind _returnvalue_4 (`|SpawnActorFromClass` "/Game/HorrorDungeon/AbilitySystem/Player/Abilities/Warrior/Physical/RadiantStrike/BP_RadiantExplosion.BP_RadiantExplosion_C" (`KismetMathLibrary.MakeTransform` _array_element) "AdjustIfPossibleButAlwaysSpawn" "MultiplyWithRoot" null null))
                          (`Actor.SetOwner` _returnvalue_4 _returnvalue)
                          (set `HDProjectile.DamageEffectParams` (make `DamageEffectParams` _returnvalue "/Game/HorrorDungeon/AbilitySystem/Player/Effects/Debuffs/GE_Damage.GE_Damage_C" (`self.GetAbilitySystemComponentFromActorInfo`) null 25.0 1.0 (struct :`TagName` "Damage.Physical") 0.0 0.0 0.0 0.0 0.0 (0.0 0.0 0.0) 0.0 0.0 (0.0 0.0 0.0) false 50.0 25.0 _array_element) _returnvalue_4))
                        (`self.K2_EndAbility`))))
                  (:`EventReceived`
                    (`/Game/HorrorDungeon/Actor/Weapons/Melee/BP_MeleeWeapon.MeshChange` (`self.Melee Weapon`) false))))
              (:`EventReceived`
                (`MeleeWeapon.AbilityHandleCollision` (`self.Melee Weapon`) true))))
          (:`EventReceived`
            (`/Game/HorrorDungeon/Actor/Weapons/Melee/BP_MeleeWeapon.MeshChange` (`self.Melee Weapon`) true)))))
    (else
      (`self.K2_EndAbility`))))