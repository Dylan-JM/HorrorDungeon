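; Gameplay ability for the player Warrior's default melee attack, run only when the equipped weapon passes the correct-weapon check.
; It sets damage, commits, then plays the first tagged attack montage from the equipped weapon.
; Montage gameplay events toggle weapon collision through avatar messages, enabling it on the montage's socket tag.
; The ability ends on montage completion or failed checks; interruption is not handled.
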(event `self.K2_ActivateAbility`
  (`self.StoreOwnerVariables`)
  (bind _returnvalue (`self.IsCorrectWeapon` "/Script/HorrorDungeon.BaseWeapon"))
  (if _returnvalue
    (`self.SetDamage`)
    (bind _returnvalue_2 (message `CombatInterface.GetEquippedWeapon1` (`self.OwnerCharacter`)))
    (`/Engine/EditorBlueprintResources/StandardMacros.IsValid` _returnvalue_2
      (:`Is Valid`
        (`self.K2_CommitAbility`)
        (bind (_returnvalue_montage _returnvalue_montagetag _returnvalue_sockettag) (break `TaggedMontage` (`self.GetTaggedMontage` (`BaseWeapon.AttackMontages` _returnvalue_2) (struct :`TagName` "Montage.Attack.1"))))
        (`AbilityTask_PlayMontageAndWait.CreatePlayMontageAndWaitProxy` "None" _returnvalue_montage 1.0 "None" false
          (:`then`
            (`AbilityTask_WaitGameplayEvent.WaitGameplayEvent` (struct :`TagName` "Montage.Attack") null
              (:`then`
                (`AbilityTask_WaitGameplayEvent.WaitGameplayEvent` (struct :`TagName` "Montage.Attack.DisableCollision") null
                  (:`EventReceived`
                    (message `CombatInterface.DisableWeaponCollision` (`self.GetAvatarActorFromActorInfo`)))))
              (:`EventReceived`
                (message `CombatInterface.EnableWeaponCollision` (`self.GetAvatarActorFromActorInfo`) _returnvalue_sockettag))))
          (:`OnCompleted`
            (`self.K2_EndAbility`))))
      (:`Is Not Valid`
        (`self.K2_EndAbility`)))
    (else
      (`self.K2_EndAbility`))))