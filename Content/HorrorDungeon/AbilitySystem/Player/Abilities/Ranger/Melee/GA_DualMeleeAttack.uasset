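; Ranger melee Gameplay Ability that performs light or heavy attacks with the equipped weapon, with separate montages for dual and single wielding.
; On input release, hold time selects a light attack or a double-damage heavy attack with an extra cost commit.
; Pressing again during a light attack chains a second swing at the attack-end event, using a hardcoded reversed dagger montage when single wielding.
; Montage gameplay events toggle weapon collision on tagged sockets.
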(event `self.K2_ActivateAbility`
  (bind (_damage_value _damage_curve _damage_registrytype) (break `ScalableFloat` (`self.Damage`)))
  (bind (_damage_value_2 _damage_curve_2 _damage_registrytype_2) (break `ScalableFloat` (`self.Damage`)))
  (bind (_damage_value_3 _damage_curve_3 _damage_registrytype_3) (break `ScalableFloat` (`self.Damage`)))
  (bind (_damage_value_4 _damage_curve_4 _damage_registrytype_4) (break `ScalableFloat` (`self.Damage`)))
  (`self.StoreOwnerVariables`)
  (bind _returnvalue (`self.IsCorrectWeapon` "/Script/HorrorDungeon.MeleeWeapon"))
  (if _returnvalue
    (bind _returnvalue_2 (message `CombatInterface.GetEquippedWeapon1` (`self.OwnerCharacter`)))
    (bind _asmelee_weapon (cast `MeleeWeapon` _returnvalue_2))
    (bind _output_get (set `self.MeleeWeapon` _asmelee_weapon))
    (bind (_asynctaskproxy _timeheld) (`AbilityTask_WaitInputRelease.WaitInputRelease` false)
      (:`OnRelease`
        (`self.K2_CommitAbility`)
        (if (`self.IsDualWielding`)
          (if (< _timeheld 0.25)
            (set `self.Damage` (make `ScalableFloat` 1.0 _damage_curve _damage_registrytype))
            (`self.SetDamage`)
            (bind _attackmontages (`BaseWeapon.AttackMontages` _output_get))
            (bind (_returnvalue_montage _returnvalue_montagetag _returnvalue_sockettag) (break `TaggedMontage` (`self.GetTaggedMontage` _attackmontages (struct :`TagName` "Montage.Attack.1"))))
            (`AbilityTask_PlayMontageAndWait.CreatePlayMontageAndWaitProxy` "None" _returnvalue_montage 1.0 "None" false
              (:`then`
                (`AbilityTask_WaitGameplayEvent.WaitGameplayEvent` (struct :`TagName` "Montage.Attack") null
                  (:`then`
                    (`AbilityTask_WaitGameplayEvent.WaitGameplayEvent` (struct :`TagName` "Montage.Attack.DisableCollision") null
                      (:`then`
                        (`AbilityTask_WaitInputPress.WaitInputPress` false
                          (:`OnPress`
                            (`AbilityTask_WaitGameplayEvent.WaitGameplayEvent` (struct :`TagName` "Montage.Attack.End") null
                              (:`EventReceived`
                                (`self.K2_CommitAbility`)
                                (bind (_returnvalue_montage_2 _returnvalue_montagetag_2 _returnvalue_sockettag_2) (break `TaggedMontage` (`self.GetTaggedMontage` _attackmontages (struct :`TagName` "Montage.Attack.2"))))
                                (`AbilityTask_PlayMontageAndWait.CreatePlayMontageAndWaitProxy` "None" _returnvalue_montage_2 1.0 "None" false
                                  (:`then`
                                    (`AbilityTask_WaitGameplayEvent.WaitGameplayEvent` (struct :`TagName` "Montage.Attack") null
                                      (:`EventReceived`
                                        (message `CombatInterface.EnableWeaponCollision` (`self.GetAvatarActorFromActorInfo`) _returnvalue_sockettag_2))))
                                  (:`OnCompleted`
                                    (message `CombatInterface.DisableWeaponCollision` (`self.GetAvatarActorFromActorInfo`) :!label _label)
                                    (`self.K2_EndAbility`))
                                  (:`OnInterrupted`
                                    (goto _label))
                                  (:`OnCancelled`
                                    (goto _label))))))))
                      (:`EventReceived`
                        (message `CombatInterface.DisableWeaponCollision` (`self.GetAvatarActorFromActorInfo`)))))
                  (:`EventReceived`
                    (message `CombatInterface.EnableWeaponCollision` (`self.GetAvatarActorFromActorInfo`) _returnvalue_sockettag))))
              (:`OnCompleted`
                (`self.K2_EndAbility`))
              (:`OnInterrupted`
                (message `CombatInterface.DisableWeaponCollision` (`self.GetAvatarActorFromActorInfo`) :!label _label_2))
              (:`OnCancelled`
                (goto _label_2)))
            (else
              (set `self.Damage` (make `ScalableFloat` 2.0 _damage_curve_2 _damage_registrytype_2))
              (`self.SetDamage`)
              (`self.K2_CommitAbilityCost` false)
              (bind (_returnvalue_montage_3 _returnvalue_montagetag_3 _returnvalue_sockettag_3) (break `TaggedMontage` (`self.GetTaggedMontage` _attackmontages (struct :`TagName` "Montage.Attack.3"))))
              (`AbilityTask_PlayMontageAndWait.CreatePlayMontageAndWaitProxy` "None" _returnvalue_montage_3 1.0 "None" false
                (:`then`
                  (`AbilityTask_WaitGameplayEvent.WaitGameplayEvent` (struct :`TagName` "Montage.Attack") null
                    (:`then`
                      (`AbilityTask_WaitGameplayEvent.WaitGameplayEvent` (struct :`TagName` "Montage.Attack.DisableCollision") null
                        (:`EventReceived`
                          (message `CombatInterface.DisableWeaponCollision` (`self.GetAvatarActorFromActorInfo`)))))
                    (:`EventReceived`
                      (message `CombatInterface.EnableWeaponCollision` (`self.GetAvatarActorFromActorInfo`) _returnvalue_sockettag_3)
                      (`KismetArrayLibrary.Array_Clear` (`BaseWeapon.ActorsToIgnore` (`self.MeleeWeapon`))))))
                (:`OnCompleted`
                  (message `CombatInterface.DisableWeaponCollision` (`self.GetAvatarActorFromActorInfo`) :!label _label_3)
                  (`self.K2_EndAbility`))
                (:`OnInterrupted`
                  (goto _label_3))
                (:`OnCancelled`
                  (goto _label_3)))))
          (elif (< _timeheld 0.25)
            (set `self.Damage` (make `ScalableFloat` 1.0 _damage_curve_3 _damage_registrytype_3))
            (`self.SetDamage`)
            (bind _attackmontages_2 (`BaseWeapon.AttackMontages` _output_get))
            (bind (_returnvalue_montage_4 _returnvalue_montagetag_4 _returnvalue_sockettag_4) (break `TaggedMontage` (`self.GetTaggedMontage` _attackmontages_2 (struct :`TagName` "Montage.Attack.1"))))
            (`AbilityTask_PlayMontageAndWait.CreatePlayMontageAndWaitProxy` "None" _returnvalue_montage_4 1.0 "None" false
              (:`then`
                (`AbilityTask_WaitGameplayEvent.WaitGameplayEvent` (struct :`TagName` "Montage.Attack") null
                  (:`then`
                    (`AbilityTask_WaitGameplayEvent.WaitGameplayEvent` (struct :`TagName` "Montage.Attack.DisableCollision") null
                      (:`then`
                        (`AbilityTask_WaitInputPress.WaitInputPress` false
                          (:`OnPress`
                            (`AbilityTask_WaitGameplayEvent.WaitGameplayEvent` (struct :`TagName` "Montage.Attack.End") null
                              (:`EventReceived`
                                (`self.K2_CommitAbility`)
                                (`AbilityTask_PlayMontageAndWait.CreatePlayMontageAndWaitProxy` "None" "/Game/Assets/Characters/Mannequins/MyAnimations/Montages/AM_DaggerAttackReversed.AM_DaggerAttackReversed" 1.0 "None" false 1.0 1.0
                                  (:`then`
                                    (`AbilityTask_WaitGameplayEvent.WaitGameplayEvent` (struct :`TagName` "Montage.Attack") null
                                      (:`EventReceived`
                                        (message `CombatInterface.EnableWeaponCollision` (`self.GetAvatarActorFromActorInfo`) _returnvalue_sockettag_4))))
                                  (:`OnCompleted`
                                    (message `CombatInterface.DisableWeaponCollision` (`self.GetAvatarActorFromActorInfo`) :!label _label_4)
                                    (`self.K2_EndAbility`))
                                  (:`OnInterrupted`
                                    (goto _label_4))
                                  (:`OnCancelled`
                                    (goto _label_4))))))))
                      (:`EventReceived`
                        (message `CombatInterface.DisableWeaponCollision` (`self.GetAvatarActorFromActorInfo`)))))
                  (:`EventReceived`
                    (message `CombatInterface.EnableWeaponCollision` (`self.GetAvatarActorFromActorInfo`) _returnvalue_sockettag_4))))
              (:`OnCompleted`
                (`self.K2_EndAbility`))
              (:`OnInterrupted`
                (message `CombatInterface.DisableWeaponCollision` (`self.GetAvatarActorFromActorInfo`) :!label _label_5))
              (:`OnCancelled`
                (goto _label_5)))
            (else
              (set `self.Damage` (make `ScalableFloat` 2.0 _damage_curve_4 _damage_registrytype_4))
              (`self.SetDamage`)
              (`self.K2_CommitAbilityCost` false)
              (bind (_returnvalue_montage_5 _returnvalue_montagetag_5 _returnvalue_sockettag_5) (break `TaggedMontage` (`self.GetTaggedMontage` _attackmontages_2 (struct :`TagName` "Montage.Attack.4"))))
              (`AbilityTask_PlayMontageAndWait.CreatePlayMontageAndWaitProxy` "None" _returnvalue_montage_5 1.0 "None" false
                (:`then`
                  (`AbilityTask_WaitGameplayEvent.WaitGameplayEvent` (struct :`TagName` "Montage.Attack") null
                    (:`then`
                      (`AbilityTask_WaitGameplayEvent.WaitGameplayEvent` (struct :`TagName` "Montage.Attack.DisableCollision") null
                        (:`EventReceived`
                          (message `CombatInterface.DisableWeaponCollision` (`self.GetAvatarActorFromActorInfo`)))))
                    (:`EventReceived`
                      (message `CombatInterface.EnableWeaponCollision` (`self.GetAvatarActorFromActorInfo`) _returnvalue_sockettag_5)
                      (`KismetArrayLibrary.Array_Clear` (`BaseWeapon.ActorsToIgnore` (`self.MeleeWeapon`))))))
                (:`OnCompleted`
                  (message `CombatInterface.DisableWeaponCollision` (`self.GetAvatarActorFromActorInfo`) :!label _label_6)
                  (`self.K2_EndAbility`))
                (:`OnInterrupted`
                  (goto _label_6))
                (:`OnCancelled`
                  (goto _label_6))))))))
    (else
      (`self.K2_EndAbility`))))