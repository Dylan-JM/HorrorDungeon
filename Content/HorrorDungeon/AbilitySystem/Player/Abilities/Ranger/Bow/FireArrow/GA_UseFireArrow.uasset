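; Ranger gameplay ability that switches the owning character to fire arrows for the bow.
; On activation it commits, sets the owner's UseFireArrow flag and fetches equipped weapon 1 as a BP_Bow.
; If the bow's arrow mesh is visible, it activates the fire component, and the locally controlled instance also calls ServerActivateFire on the bow.
; It then ends immediately, except when no valid weapon is found, where EndAbility is never called.
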(event `self.K2_ActivateAbility`
  (bind _ownercharacter (`self.OwnerCharacter`))
  (`self.K2_CommitAbility`)
  (`self.StoreOwnerVariables`)
  (set `BaseCharacter.bUseFireArrow` true _ownercharacter)
  (bind _returnvalue (message `CombatInterface.GetEquippedWeapon1` _ownercharacter))
  (`/Engine/EditorBlueprintResources/StandardMacros.IsValid` _returnvalue
    (:`Is Valid`
      (bind _asbp_bow (cast `/Game/HorrorDungeon/Actor/Weapons/Bow/BP_Bow` _returnvalue)
        (:`then`
          (set `self.Bow` _asbp_bow)
          (if (`SceneComponent.bVisible` (`Bow.ArrowMesh` _asbp_bow))
            (`ActorComponent.Activate` (`Bow.FireComponent` _asbp_bow) false)
            (`self.IsLocallyControlled`
              (:`True`
                (`/Game/HorrorDungeon/Actor/Weapons/Bow/BP_Bow.ServerActivateFire` (`self.Bow`) true)
                (`self.K2_EndAbility`))
              (:`False`
                (`self.K2_EndAbility`)))
            (else
              (`self.K2_EndAbility`))))
        (:`CastFailed`
          (`self.K2_EndAbility`))))))