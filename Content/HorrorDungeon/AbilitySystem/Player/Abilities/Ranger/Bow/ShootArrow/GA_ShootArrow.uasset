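; Ranger bow ability that draws while input is held and fires an arrow on release.
; It requires an equipped bow and inventory arrows, consuming one per shot, committing cooldown and turning the player toward the hit target.
; A montage gameplay event spawns the projectile, then arrow visibility is restored from remaining stock after a short delay.
; Server events replay montages, sync arrow visibility and switch projectile and damage to fire when a fire arrow is primed.
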(event `ServerPlayMontage`
  (params (MontageToPlay :type "AnimMontage Object Reference"))
  (`AbilityTask_PlayMontageAndWait.CreatePlayMontageAndWaitProxy` "None" MontageToPlay))

(event `self.K2_ActivateAbility`
  (bind (_icon _iconrotated _itemclass _dimensions _itemtype _brotated _bistwohanded _maxstacks _currentstacks) (break `ItemObjectValues` (`ItemObject.ItemObjectValues` (`self.Arrow`))))
  (message `CombatInterface.SetIsAttacking` (`self.GetAvatarActorFromActorInfo`) false)
  (`self.StoreOwnerVariables`)
  (bind _returnvalue (`self.IsCorrectWeapon` "/Script/HorrorDungeon.Bow"))
  (bind _returnvalue_2 (message `CombatInterface.GetEquippedWeapon1` (`self.OwnerCharacter`)))
  (bind _asbp_bow (cast `/Game/HorrorDungeon/Actor/Weapons/Bow/BP_Bow` _returnvalue_2)
    (:`then`
      (set `self.Bow` _asbp_bow)
      (if _returnvalue
        (bind _asbp_inventory_component_2 (cast `/Game/HorrorDungeon/Player/Components/BP_InventoryComponent2` (`BaseCharacter.InventoryComponent` (`self.OwnerCharacter`))))
        (bind _output_get (set `self.BPInventoryComponent` _asbp_inventory_component_2))
        (bind _foundarrow (`self.FindArrowInInventory` (`/Game/HorrorDungeon/Player/Components/BP_InventoryComponent2.ItemsBP` _output_get)))
        (if _foundarrow
          (`AbilityTask_WaitInputRelease.WaitInputRelease` false
            (:`then`
              (`AbilityTask_PlayMontageAndWait.CreatePlayMontageAndWaitProxy` "None" "/Game/Assets/Characters/Mannequins/MyAnimations/Animations/Bow/AM_DrawBow.AM_DrawBow"
                (:`then`
                  (`self.ServerPlayMontage` "/Game/Assets/Characters/Mannequins/MyAnimations/Animations/Bow/AM_DrawBow.AM_DrawBow"))))
            (:`OnRelease`
              (if (> (`.CurrentStacks` (break `ItemObjectValues` (`ItemObject.ItemObjectValues` (`self.Arrow`)))) 1)
                (set `ItemObject.ItemObjectValues` (make `ItemObjectValues` _icon _iconrotated _itemclass _dimensions _itemtype false _bistwohanded _maxstacks (- _currentstacks 1)) (`self.Arrow`))
                (`/Game/HorrorDungeon/Player/Components/BP_InventoryComponent2.OnInventoryChanged` (`self.BPInventoryComponent`))
                (else
                  (`/Game/HorrorDungeon/Player/Components/BP_InventoryComponent2.RemoveItem` (`self.BPInventoryComponent`) (`self.Arrow`))))
              (set `BaseCharacter.bShouldHoldBowString` false (`self.OwnerCharacter`))
              (`self.K2_CommitAbilityCooldown` false)
              (if (`BaseCharacter.bUseFireArrow` (`self.OwnerCharacter`))
                (set `BaseCharacter.bUseFireArrow` false (`self.OwnerCharacter`))
                (`ActorComponent.Deactivate` (`Bow.FireComponent` (`self.Bow`)))
                (`self.ServerSetDamageVariables`))
              (`self.RotatePlayer`)
              (`AbilityTask_PlayMontageAndWait.CreatePlayMontageAndWaitProxy` "None" "/Game/Assets/Animations/Archery/Montages/Player/M_ShootArrow.M_ShootArrow"
                (:`then`
                  (`self.ServerPlayMontage` "/Game/Assets/Animations/Archery/Montages/Player/M_ShootArrow.M_ShootArrow")
                  (`AbilityTask_WaitGameplayEvent.WaitGameplayEvent` (struct :`TagName` "Montage.Attack.1") null
                    (:`EventReceived`
                      (`self.SpawnProjectile`)
                      (`SceneComponent.SetVisibility` (`Bow.ArrowMesh` (`self.Bow`)) false false)
                      (`self.ServerSetArrowVisibility` false (`self.Bow`)))))
                (:`OnCompleted`
                  (`KismetSystemLibrary.Delay` 0.6 :!label _label)
                  (set `BaseCharacter.bShouldHoldBowString` true (`self.OwnerCharacter`))
                  (bind _foundarrow_2 (`self.FindArrowInInventory` (`/Game/HorrorDungeon/Player/Components/BP_InventoryComponent2.ItemsBP` (`self.BPInventoryComponent`))))
                  (`SceneComponent.SetVisibility` (`Bow.ArrowMesh` (`self.Bow`)) _foundarrow_2 false)
                  (`self.ServerSetArrowVisibility` _foundarrow_2 (`self.Bow`) (`BaseCharacter.bUseFireArrow` (`self.OwnerCharacter`)))
                  (`self.K2_EndAbility`))
                (:`OnInterrupted`
                  (goto _label)))))
          (else
            (`self.K2_EndAbility`)))
        (else
          (`self.K2_EndAbility`))))
    (:`CastFailed`
      (`self.K2_EndAbility`))))

(event `ServerSetDamageVariables`
  (set `self.DamageType` (struct :`TagName` "Damage.Fire"))
  (set `self.DebuffChance` 100.0)
  (set `self.ProjectileClass` "/Game/HorrorDungeon/AbilitySystem/Player/Abilities/Ranger/Bow/FireArrow/BP_FireArrow.BP_FireArrow_C"))

(event `ServerSetArrowVisibility`
  (params (NewVisibility :type Boolean) (InBow :type "/Game/HorrorDungeon/Actor/Weapons/Bow/BP_Bow Object Reference") (ActivateFire :type Boolean))
  (`SceneComponent.SetVisibility` (`Bow.ArrowMesh` InBow) NewVisibility false)
  (`/Game/HorrorDungeon/Actor/Weapons/Bow/BP_Bow.MultiActivateFire` InBow ActivateFire))

(fn `FindArrowInInventory`
  (params (Array :type "Array of ItemObject Object Reference"))
  (returns (FoundArrow :type Boolean))
  (for _array_element Array
    (`/Engine/EditorBlueprintResources/StandardMacros.IsValid` _array_element
      (:`Is Valid`
        (if (== (`.ItemClass` (break `ItemObjectValues` (`ItemObject.ItemObjectValues` _array_element))) "/Game/HorrorDungeon/Actor/Weapons/Bow/BP_InventoryArrow.BP_InventoryArrow_C")
          (set `self.Arrow` _array_element)
          (return true)))))
  (return false))

(fn `RotatePlayer`
  (bind (_returnvalue_roll _returnvalue_pitch _returnvalue_yaw) (`KismetMathLibrary.BreakRotator` (`KismetMathLibrary.FindLookAtRotation` (`SceneComponent.K2_GetComponentLocation` (`Character.CapsuleComponent` (`self.OwnerCharacter`))) (`self.HitTargetLoc`))))
  (`SceneComponent.K2_SetWorldRotation` (`Character.CapsuleComponent` (`self.OwnerCharacter`)) (`KismetMathLibrary.MakeRotator` 0.0 0.0 _returnvalue_yaw) false false))