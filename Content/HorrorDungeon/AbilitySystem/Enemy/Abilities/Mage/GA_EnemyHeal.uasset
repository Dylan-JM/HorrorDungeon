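; Enemy mage heal ability that plays the avatar's tagged heal montage and spawns a BP_HealArea during it.
; A visibility trace from the avatar places the area at its hit, or stops the montage on a miss; its end point multiplies the location rather than offsetting downward.
; When the montage completes, interrupts or cancels, it fires the heal-finished delegate, but destroys the area and ends the ability only if that area is valid.
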(event `self.K2_ActivateAbility`
  (bind _returnvalue (`Actor.K2_GetActorLocation` (`self.GetAvatarActorFromActorInfo`)))
  (bind _asbase_character (cast `BaseCharacter` (`self.GetAvatarActorFromActorInfo`))
    (:`then`
      (bind _output_get (set `self.EnemyCharacter` _asbase_character))
      (bind _returnvalue_2 (message `CombatInterface.GetAbilityMontages` _output_get))
      (`AbilityTask_PlayMontageAndWait.CreatePlayMontageAndWaitProxy` "None" (`.Montage` (break `TaggedMontage` (`self.GetTaggedMontage` _returnvalue_2 (struct :`TagName` "Montage.Defence.Heal")))) ; Make montage to player variable if want to use this with not just enemy character model
        (:`then`
          (bind (_outhit _returnvalue_3) (`KismetSystemLibrary.LineTraceSingle` _returnvalue (* _returnvalue (0.0 0.0 -1000.0)) "TraceTypeQuery1"))
          (if _returnvalue_3
            (bind _returnvalue_4 (`|SpawnActorFromClass` "/Game/HorrorDungeon/Actor/AOE_Status/BP_HealArea.BP_HealArea_C" (`KismetMathLibrary.Conv_VectorToTransform` (`.Location` (`GameplayStatics.BreakHitResult` _outhit))) "Undefined" "MultiplyWithRoot" null null null))
            (set `self.HealArea` _returnvalue_4)
            (else
              (`self.MontageStop` -1.0))))
        (:`OnCompleted`
          (`BaseCharacter.HealFinishedDelegate` (`self.EnemyCharacter`) :!label _label)
          (bind _healarea (`self.HealArea`)
            (:`then`
              (`Actor.K2_DestroyActor` _healarea)
              (`self.K2_EndAbility`))
            (:`else`)))
        (:`OnInterrupted`
          (goto _label))
        (:`OnCancelled`
          (goto _label))))
    (:`CastFailed`
      (goto _label))))