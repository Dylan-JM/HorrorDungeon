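; Enemy mage gameplay ability that casts a Fire Bolt at the avatar's current combat target.
; It updates the facing target, then plays the montage tagged Montage.Attack.1 from the avatar's ability montages.
; A Fire Bolt montage gameplay event spawns the projectile.
; When the montage completes, is interrupted or is cancelled, it notifies the avatar of attack end, fires BP_EnemyBase's attack-finished delegate and ends the ability.
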(event `self.K2_ActivateAbility`
  (bind _returnvalue (`self.GetAvatarActorFromActorInfo`))
  (bind _returnvalue_2 (message `EnemyInterface.GetCombatTarget` _returnvalue))
  (set `self.CombatTarget` _returnvalue_2)
  (message `CombatInterface.UpdateFacingTarget` _returnvalue (`Actor.K2_GetActorLocation` _returnvalue_2))
  (bind _returnvalue_3 (message `CombatInterface.GetAbilityMontages` (`self.GetAvatarActorFromActorInfo`)))
  (`AbilityTask_PlayMontageAndWait.CreatePlayMontageAndWaitProxy` "None" (`.Montage` (break `TaggedMontage` (`self.GetTaggedMontage` _returnvalue_3 (struct :`TagName` "Montage.Attack.1")))) 1.0 "None" false
    (:`then`
      (`AbilityTask_WaitGameplayEvent.WaitGameplayEvent` (struct :`TagName` "Event.Montage.FireBolt") null
        (:`EventReceived`
          (`self.SpawnProjectile`))))
    (:`OnCompleted`
      (message `EnemyInterface.AttackEnd` (`self.GetAvatarActorFromActorInfo`) (`self.CombatTarget`) :!label _label)
      (bind _asbp_enemy_base (cast `/Game/HorrorDungeon/Enemy/EnemyTypes/BP_EnemyBase` (`self.GetAvatarActorFromActorInfo`)))
      (`BaseCharacter.AttackFinishedDelegate` _asbp_enemy_base)
      (`self.K2_EndAbility`))
    (:`OnInterrupted`
      (goto _label))
    (:`OnCancelled`
      (goto _label))))