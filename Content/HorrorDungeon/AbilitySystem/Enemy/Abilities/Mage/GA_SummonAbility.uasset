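; Gameplay ability for the enemy mage that summons random minions at shuffled spawn locations.
; Activation plays a ground-summon effect at every location and a summon montage, whose gameplay event starts a Delay-driven loop that staggers spawns and gives each minion a default controller.
; The caster's minion count rises per spawn and falls through bound death delegates.
; After the last spawn, it signals attack end to the caster.
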(event `self.K2_ActivateAbility`
  (bind _returnvalue (+ (`|GetArrayItem` (`self.SpawnLocations`) (`self.SpawnLocationIndex`)) (0.0 0.0 88.0)))
  (bind _returnvalue_2 (message `EnemyInterface.GetCombatTarget` (`self.GetAvatarActorFromActorInfo`)))
  (set `self.CombatTarget` _returnvalue_2)
  (bind _returnvalue_3 (`self.GetSpawnLocations`))
  (bind _output_get (set `self.SpawnLocations` _returnvalue_3))
  (`KismetArrayLibrary.Array_Shuffle` _output_get)
  (for _array_element _output_get
    (`NiagaraFunctionLibrary.SpawnSystemAtLocation` "/Game/Assets/Effects/Combat/NS_GroundSummon.NS_GroundSummon" _array_element))
  (`AbilityTask_PlayMontageAndWait.CreatePlayMontageAndWaitProxy` "None" "/Game/Assets/Animations/Magic/Montages/Player/M_MG_SummonItem.M_MG_SummonItem"
    (:`then`
      (`AbilityTask_WaitGameplayEvent.WaitGameplayEvent` (struct :`TagName` "Montage.Attack.1") null
        (:`EventReceived`
          (if (< (`self.SpawnLocationIndex`) (`KismetArrayLibrary.Array_Length` (`self.SpawnLocations`))) :!label _label
            (bind _returnvalue_4 (`|SpawnActorFromClass` (`self.GetRandomMinionClass`) (`KismetMathLibrary.MakeTransform` _returnvalue (`KismetMathLibrary.FindLookAtRotation` (`Actor.K2_GetActorLocation` (`self.GetAvatarActorFromActorInfo`)) _returnvalue)) "AlwaysSpawn" "MultiplyWithRoot" null null))
            (bind _asbase_character (cast `BaseCharacter` _returnvalue_4))
            (add `BaseCharacter.OnDeathDelegate` _asbase_character (delegate `OnMinionDied`))
            (`Pawn.SpawnDefaultController` _returnvalue_4)
            (message `CombatInterface.IncrementMinionCount` (`self.GetAvatarActorFromActorInfo`) 1)
            (`/Engine/EditorBlueprintResources/StandardMacros.IncrementInt` (`self.SpawnLocationIndex`)
              (:`  `
                (`KismetSystemLibrary.Delay` 0.2)
                (goto _label)))
            (else
              (message `EnemyInterface.AttackEnd` (`self.GetAvatarActorFromActorInfo`) (`self.CombatTarget`))
              (bind _asbp_enemy_base (cast `/Game/HorrorDungeon/Enemy/EnemyTypes/BP_EnemyBase` (`self.GetAvatarActorFromActorInfo`)))
              (`BaseCharacter.AttackFinishedDelegate` _asbp_enemy_base))))))))

(event `OnMinionDied`
  (params (DeadActor :type "Actor Object Reference"))
  (message `CombatInterface.IncrementMinionCount` (`self.GetAvatarActorFromActorInfo`) -1))