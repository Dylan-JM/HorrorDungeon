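; Boss enemy ability that spawns a temporary floating platform at the hit point of a line trace from the boss's location.
; When the platform's float timeline finishes, a timer holds it for a few seconds before telling it to stop floating.
; When the timeline finishes again, or if the platform became invalid, the ability signals attack finished, destroys the platform and ends.
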(event `self.K2_ActivateAbility`
  (bind _returnvalue (`self.GetAvatarActorFromActorInfo`))
  (bind _returnvalue_2 (`Actor.K2_GetActorLocation` _returnvalue))
  (bind _asbp_enemy_base (cast `/Game/HorrorDungeon/Enemy/EnemyTypes/BP_EnemyBase` _returnvalue))
  (set `self.Enemy` _asbp_enemy_base)
  (bind _outhit (`KismetSystemLibrary.LineTraceSingle` _returnvalue_2 (* _returnvalue_2 (0.0 0.0 -1000.0)) "TraceTypeQuery1"))
  (bind _returnvalue_3 (`|SpawnActorFromClass` "/Game/HorrorDungeon/Enemy/EnemyTypes/Boss/BP_FloatingPlatform.BP_FloatingPlatform_C" (`KismetMathLibrary.MakeTransform` (`.Location` (`GameplayStatics.BreakHitResult` _outhit))) "Undefined" "MultiplyWithRoot" null null))
  (bind _output_get (set `self.FloatingPlatform` _returnvalue_3))
  (add `/Game/HorrorDungeon/Enemy/EnemyTypes/Boss/BP_FloatingPlatform.OnFloatTimelineFinished` _output_get (delegate `FloatTimelineFinished`)))

(event `FloatTimelineFinished`
  (remove `/Game/HorrorDungeon/Enemy/EnemyTypes/Boss/BP_FloatingPlatform.OnFloatTimelineFinished` (`self.FloatingPlatform`) (delegate `FloatTimelineFinished`))
  (bind _returnvalue (`KismetSystemLibrary.K2_SetTimerDelegate` (delegate `StopFloat`) 6.5))
  (set `self.FloatPlatformTimer` _returnvalue))

(event `StopFloat`
  (bind _floatingplatform (`self.FloatingPlatform`)
    (:`then`
      (`/Game/HorrorDungeon/Enemy/EnemyTypes/Boss/BP_FloatingPlatform.StopFloating` _floatingplatform)
      (add `/Game/HorrorDungeon/Enemy/EnemyTypes/Boss/BP_FloatingPlatform.OnFloatTimelineFinished` _floatingplatform (delegate `Float Finished`)))
    (:`else`
      (`KismetSystemLibrary.DelayUntilNextTick`)
      (`BaseCharacter.AttackFinishedDelegate` (`self.Enemy`) :!label _label)
      (`Actor.K2_DestroyActor` (`self.FloatingPlatform`))
      (`self.K2_EndAbility`))))

(event `Float Finished`
  (remove `/Game/HorrorDungeon/Enemy/EnemyTypes/Boss/BP_FloatingPlatform.OnFloatTimelineFinished` (`self.FloatingPlatform`) (delegate `Float Finished`))
  (goto _label))