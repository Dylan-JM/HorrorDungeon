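; Boss gameplay ability that leaps at the combat target with a weapon attack and ground smash.
; It faces the target and plays a tagged attack montage, whose gameplay events trigger the jump, toggle weapon collision and spawn BP_GroundSmash with damage parameters.
; The jump launches the boss on a suggested projectile arc scaled by target distance, stopping movement on landing.
; Montage completion, interruption or cancellation notifies attack end and ends the ability.
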(event `self.K2_ActivateAbility`
  (bind _returnvalue (`self.GetAvatarActorFromActorInfo`))
  (bind _asbp_enemy_base (cast `/Game/HorrorDungeon/Enemy/EnemyTypes/BP_EnemyBase` (`self.GetAvatarActorFromActorInfo`)))
  (set `self.ControlledPawn` _asbp_enemy_base)
  (`self.SetDamage`)
  (bind _returnvalue_2 (message `EnemyInterface.GetCombatTarget` (`self.GetAvatarActorFromActorInfo`)))
  (set `self.CombatTarget` _returnvalue_2)
  (message `CombatInterface.UpdateFacingTarget` (`self.GetAvatarActorFromActorInfo`) (`Actor.K2_GetActorLocation` (`self.CombatTarget`)))
  (bind _returnvalue_3 (message `CombatInterface.GetAbilityMontages` (`self.GetAvatarActorFromActorInfo`)))
  (bind (_montage _montagetag _sockettag) (break `TaggedMontage` (`self.GetTaggedMontage` _returnvalue_3 (struct :`TagName` "Montage.Attack.5"))))
  (`AbilityTask_PlayMontageAndWait.CreatePlayMontageAndWaitProxy` "None" _montage 1.0 "None" false
    (:`then`
      (`AbilityTask_WaitGameplayEvent.WaitGameplayEvent` (struct :`TagName` "Montage.Jump") null
        (:`then`
          (`AbilityTask_WaitGameplayEvent.WaitGameplayEvent` (struct :`TagName` "Montage.Attack") null
            (:`then`
              (`AbilityTask_WaitGameplayEvent.WaitGameplayEvent` (struct :`TagName` "Montage.Attack.DisableCollision") null
                (:`then`
                  (`AbilityTask_WaitGameplayEvent.WaitGameplayEvent` (struct :`TagName` "Montage.Attack.1") null
                    (:`EventReceived`
                      (bind _returnvalue_4 (`|SpawnActorFromClass` "/Game/HorrorDungeon/AbilitySystem/Player/Abilities/Warrior/Physical/GroundSmash/BP_GroundSmash.BP_GroundSmash_C" (`KismetMathLibrary.Conv_VectorToTransform` (`Actor.K2_GetActorLocation` (`self.GetAvatarActorFromActorInfo`))) "Undefined" "MultiplyWithRoot" null null))
                      (bind _output_get (set `self.GroundSmashActor` _returnvalue_4))
                      (`Actor.SetOwner` _output_get _returnvalue)
                      (set `HDProjectile.DamageEffectParams` (make `DamageEffectParams` _returnvalue "/Game/HorrorDungeon/AbilitySystem/Player/Effects/Debuffs/GE_Damage.GE_Damage_C" (`self.GetAbilitySystemComponentFromActorInfo`) null (`self.GetDamageAtLevel`) 1.0 (struct :`TagName` "Damage.Physical") 0.0 0.0 0.0 0.0 0.0 (0.0 0.0 0.0) 0.0 0.0 (0.0 0.0 0.0) false 100.0 100.0 (`Actor.K2_GetActorLocation` _output_get)) _output_get))))
                (:`EventReceived`
                  (message `CombatInterface.DisableWeaponCollision` (`self.GetAvatarActorFromActorInfo`)))))
            (:`EventReceived`
              (message `CombatInterface.EnableWeaponCollision` (`self.GetAvatarActorFromActorInfo`) _sockettag))))
        (:`EventReceived`
          (`self.JumpToAttackTarget` (`self.CombatTarget`)))))
    (:`OnCompleted`
      (message `EnemyInterface.AttackEnd` (`self.GetAvatarActorFromActorInfo`) (`self.CombatTarget`) :!label _label)
      (`self.K2_EndAbility`))
    (:`OnInterrupted`
      (goto _label))
    (:`OnCancelled`
      (goto _label))))

(event `JumpToAttackTarget`
  (params (JumpTarget :type "Actor Object Reference"))
  (bind _controlledpawn (`self.ControlledPawn`))
  (bind (_returnvalue_x _returnvalue_y _returnvalue_z) (`KismetMathLibrary.BreakVector` (`Actor.K2_GetActorLocation` (`self.CombatTarget`))))
  (bind _outlaunchvelocity (`GameplayStatics.SuggestProjectileVelocity_CustomArc` (`Actor.K2_GetActorLocation` _controlledpawn) (`KismetMathLibrary.MakeVector` _returnvalue_x _returnvalue_y (+ _returnvalue_z 100.0)) 0.0 (`KismetMathLibrary.Lerp` 0.5 0.9 (`KismetMathLibrary.FClamp` (`KismetMathLibrary.NormalizeToRange` (`Actor.GetDistanceTo` JumpTarget (`self.GetAvatarActorFromActorInfo`)) 400.0 800.0)))))
  (`Character.LaunchCharacter` _controlledpawn _outlaunchvelocity true true)
  (add `Character.LandedDelegate` (`self.ControlledPawn`) (delegate `OnLandEvent`)))

(event `OnLandEvent`
  (params (Hit :type "HitResult Structure (by ref)"))
  (bind _controlledpawn (`self.ControlledPawn`))
  (remove `Character.LandedDelegate` _controlledpawn (delegate `OnLandEvent`))
  (`MovementComponent.StopMovementImmediately` (`Character.CharacterMovement` _controlledpawn)))