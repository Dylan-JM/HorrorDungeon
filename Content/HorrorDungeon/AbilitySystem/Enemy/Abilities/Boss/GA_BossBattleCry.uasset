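; Boss enemy battle cry ability that repeatedly drops damaging magic circles at its combat target's position.
; It plays a montage selected by the ability's first tag, and montage gameplay events start and stop a looping spawn timer.
; Each spawned BP_BattleCryCircle uses the target's X and Y and receives level-scaled damage params with itself as radial origin.
; Montage completion, interruption or cancellation notifies that the attack finished and ends the ability.
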(event `self.K2_ActivateAbility`
  (bind _asbp_enemy_base (cast `/Game/HorrorDungeon/Enemy/EnemyTypes/BP_EnemyBase` (`self.GetAvatarActorFromActorInfo`)))
  (set `self.ControlledPawn` _asbp_enemy_base)
  (bind _returnvalue (message `EnemyInterface.GetCombatTarget` (`self.GetAvatarActorFromActorInfo`)))
  (set `self.CombatTarget` _returnvalue)
  (bind _montage (`self.GetMontageByTag`))
  (`AbilityTask_PlayMontageAndWait.CreatePlayMontageAndWaitProxy` "None" _montage 1.0 "None" false
    (:`then`
      (`AbilityTask_WaitGameplayEvent.WaitGameplayEvent` (struct :`TagName` "Montage.Attack") null
        (:`then`
          (`AbilityTask_WaitGameplayEvent.WaitGameplayEvent` (struct :`TagName` "Montage.Attack.RadiantStrikeEnd") null
            (:`EventReceived`
              (`KismetSystemLibrary.K2_ClearAndInvalidateTimerHandle` (`self.SpawnExposionTimer`)))))
        (:`EventReceived`
          (bind _returnvalue_2 (`KismetSystemLibrary.K2_SetTimerDelegate` (delegate `SpawnExplosion`) 0.5 true))
          (set `self.SpawnExposionTimer` _returnvalue_2))))
    (:`OnCompleted`
      (`BaseCharacter.AttackFinishedDelegate` (`self.ControlledPawn`) :!label _label)
      (`self.K2_EndAbility`))
    (:`OnInterrupted`
      (goto _label))
    (:`OnCancelled`
      (goto _label))))

(event `SpawnExplosion`
  (bind _returnvalue_location (`KismetMathLibrary.BreakTransform` (`Actor.GetTransform` (`self.CombatTarget`))))
  (set `self.ExplosionSpawnLocation` _returnvalue_location)
  (bind _returnvalue (`|SpawnActorFromClass` "/Game/HorrorDungeon/AbilitySystem/Player/Abilities/Warrior/Battlecry/BP_BattleCryCircle.BP_BattleCryCircle_C" (`KismetMathLibrary.MakeTransform` (`KismetMathLibrary.MakeVector` (.x _returnvalue_location) (.y _returnvalue_location))) "Undefined" "MultiplyWithRoot" (`self.GetAvatarActorFromActorInfo`) (struct) null))
  (bind _output_get (set `self.MagicCircle` _returnvalue))
  (set `/Game/HorrorDungeon/AbilitySystem/Player/Abilities/Warrior/Battlecry/BP_BattleCryCircle.DamageEffectParams` (make `DamageEffectParams` (`self.GetAvatarActorFromActorInfo`) "/Game/HorrorDungeon/AbilitySystem/Player/Effects/Debuffs/GE_Damage.GE_Damage_C" (`self.GetAbilitySystemComponentFromActorInfo`) null (`self.GetDamageAtLevel`) 1.0 (struct :`TagName` "Damage.Physical") 0.0 0.0 0.0 0.0 0.0 (0.0 0.0 0.0) 0.0 0.0 (0.0 0.0 0.0) false 100.0 100.0 (`Actor.K2_GetActorLocation` _output_get)) _output_get))

(fn `GetMontageByTag`
  (returns (Montage :type "AnimMontage Object Reference") (`Montage Tag` :type "GameplayTag Structure") (`Socket Tag` :type "GameplayTag Structure"))
  (bind _returnvalue (message `CombatInterface.GetAbilityMontages` (`self.GetAvatarActorFromActorInfo`)))
  (bind (_montage _montagetag _sockettag) (break `TaggedMontage` (`self.GetTaggedMontage` _returnvalue (`|GetArrayItem` (`BlueprintGameplayTagLibrary.BreakGameplayTagContainer` (`self.GetAbilityTags`))))))
  (return _montage _montagetag _sockettag))