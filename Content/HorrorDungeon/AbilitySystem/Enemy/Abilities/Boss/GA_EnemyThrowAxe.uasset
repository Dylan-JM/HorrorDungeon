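; Boss enemy gameplay ability that throws the equipped melee weapon as a projectile at the combat target.
; It updates the facing target to the target's location, then plays the montage tagged Montage.Attack.3.
; On the Montage.Attack gameplay event it hides the weapon mesh and calls SpawnProjectile, faking the throw.
; When the montage completes, is interrupted or is cancelled, it signals attack end, reshows the weapon and ends the ability.
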(event `self.K2_ActivateAbility`
  (bind _returnvalue (`self.GetAvatarActorFromActorInfo`))
  (bind _asbp_enemy_base (cast `/Game/HorrorDungeon/Enemy/EnemyTypes/BP_EnemyBase` (`self.GetAvatarActorFromActorInfo`)))
  (bind _output_get (set `self.Enemy` _asbp_enemy_base))
  (bind _returnvalue_2 (message `CombatInterface.GetEquippedWeapon1` _output_get))
  (bind _asbp_melee_weapon (cast `/Game/HorrorDungeon/Actor/Weapons/Melee/BP_MeleeWeapon` _returnvalue_2))
  (set `self.Melee Weapon` _asbp_melee_weapon)
  (bind _returnvalue_3 (message `EnemyInterface.GetCombatTarget` _returnvalue))
  (set `self.CombatTarget` _returnvalue_3)
  (message `CombatInterface.UpdateFacingTarget` _returnvalue (`Actor.K2_GetActorLocation` _returnvalue_3))
  (bind _returnvalue_4 (message `CombatInterface.GetAbilityMontages` (`self.GetAvatarActorFromActorInfo`)))
  (`AbilityTask_PlayMontageAndWait.CreatePlayMontageAndWaitProxy` "None" (`.Montage` (break `TaggedMontage` (`self.GetTaggedMontage` _returnvalue_4 (struct :`TagName` "Montage.Attack.3")))) 1.0 "None" false
    (:`then`
      (`AbilityTask_WaitGameplayEvent.WaitGameplayEvent` (struct :`TagName` "Montage.Attack") null
        (:`EventReceived`
          (`SceneComponent.SetVisibility` (`EquippableActor.ItemMesh` (`self.Melee Weapon`)) false true)
          (`self.SpawnProjectile`))))
    (:`OnCompleted`
      (message `EnemyInterface.AttackEnd` (`self.GetAvatarActorFromActorInfo`) (`self.CombatTarget`) :!label _label)
      (bind _asbp_enemy_base_2 (cast `/Game/HorrorDungeon/Enemy/EnemyTypes/BP_EnemyBase` (`self.GetAvatarActorFromActorInfo`)))
      (`BaseCharacter.AttackFinishedDelegate` _asbp_enemy_base_2)
      (`SceneComponent.SetVisibility` (`EquippableActor.ItemMesh` (`self.Melee Weapon`)) true true)
      (`self.K2_EndAbility`))
    (:`OnInterrupted`
      (goto _label))
    (:`OnCancelled`
      (goto _label))))