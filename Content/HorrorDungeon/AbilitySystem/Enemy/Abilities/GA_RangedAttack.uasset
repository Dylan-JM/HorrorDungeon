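; Enemy ranged attack gameplay ability that turns the avatar toward its combat target and fires a projectile during an attack montage.
; It gets target and montages through messages to the avatar, then plays the montage tagged Montage.Attack.1.
; A one-shot gameplay event wait triggers SpawnProjectile, syncing the shot to an event rather than activation.
; Montage completion, interruption or cancellation notifies the avatar that the attack ended and ends the ability.
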(event `self.K2_ActivateAbility`
  (bind _returnvalue (message `EnemyInterface.GetCombatTarget` (`self.GetAvatarActorFromActorInfo`)))
  (set `self.CombatTarget` _returnvalue)
  (message `CombatInterface.UpdateFacingTarget` (`self.GetAvatarActorFromActorInfo`) (`Actor.K2_GetActorLocation` (`self.CombatTarget`)))
  (bind _returnvalue_2 (message `CombatInterface.GetAbilityMontages` (`self.GetAvatarActorFromActorInfo`)))
  (`AbilityTask_PlayMontageAndWait.CreatePlayMontageAndWaitProxy` "None" (`.Montage` (break `TaggedMontage` (`self.GetTaggedMontage` _returnvalue_2 (struct :`TagName` "Montage.Attack.1")))) 1.0 "None" false
    (:`then`
      (`AbilityTask_WaitGameplayEvent.WaitGameplayEvent` (struct) null true
        (:`EventReceived`
          (`self.SpawnProjectile`))))
    (:`OnCompleted`
      (message `EnemyInterface.AttackEnd` (`self.GetAvatarActorFromActorInfo`) (`self.CombatTarget`) :!label _label)
      (`self.K2_EndAbility`))
    (:`OnInterrupted`
      (goto _label))
    (:`OnCancelled`
      (goto _label))))