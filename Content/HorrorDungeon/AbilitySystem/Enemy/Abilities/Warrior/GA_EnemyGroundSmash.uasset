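; Enemy Warrior ground smash ability that turns the avatar toward its combat target and plays a tagged attack montage.
; When the montage attack gameplay event arrives, it spawns a BP_GroundSmash actor at the avatar's location, owned by the avatar.
; That actor receives damage effect params with level-scaled damage and its own location as radial origin.
; Montage completion, interruption or cancellation all send the attack-end message to the avatar and end the ability.
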(event `self.K2_ActivateAbility`
  (bind _returnvalue (`self.GetAvatarActorFromActorInfo`))
  (bind _returnvalue_2 (message `EnemyInterface.GetCombatTarget` (`self.GetAvatarActorFromActorInfo`)))
  (set `self.CombatTarget` _returnvalue_2)
  (message `CombatInterface.UpdateFacingTarget` (`self.GetAvatarActorFromActorInfo`) (`Actor.K2_GetActorLocation` (`self.CombatTarget`)))
  (bind _returnvalue_3 (message `CombatInterface.GetAbilityMontages` (`self.GetAvatarActorFromActorInfo`)))
  (`AbilityTask_PlayMontageAndWait.CreatePlayMontageAndWaitProxy` "None" (`.Montage` (break `TaggedMontage` (`self.GetTaggedMontage` _returnvalue_3 (struct :`TagName` "Montage.Attack.4")))) 1.0 "None" false
    (:`then`
      (`AbilityTask_WaitGameplayEvent.WaitGameplayEvent` (struct :`TagName` "Montage.Attack") null
        (:`EventReceived`
          (bind _returnvalue_4 (`|SpawnActorFromClass` "/Game/HorrorDungeon/AbilitySystem/Player/Abilities/Warrior/Physical/GroundSmash/BP_GroundSmash.BP_GroundSmash_C" (`KismetMathLibrary.Conv_VectorToTransform` (`Actor.K2_GetActorLocation` (`self.GetAvatarActorFromActorInfo`))) "Undefined" "MultiplyWithRoot" null null))
          (bind _output_get (set `self.GroundSmashActor` _returnvalue_4))
          (`Actor.SetOwner` _output_get _returnvalue)
          (set `HDProjectile.DamageEffectParams` (make `DamageEffectParams` _returnvalue "/Game/HorrorDungeon/AbilitySystem/Player/Effects/Debuffs/GE_Damage.GE_Damage_C" (`self.GetAbilitySystemComponentFromActorInfo`) null (`self.GetDamageAtLevel`) 1.0 (struct :`TagName` "Damage.Physical") 0.0 0.0 0.0 0.0 0.0 (0.0 0.0 0.0) 0.0 0.0 (0.0 0.0 0.0) false 100.0 100.0 (`Actor.K2_GetActorLocation` _output_get)) _output_get))))
    (:`OnCompleted`
      (message `EnemyInterface.AttackEnd` (`self.GetAvatarActorFromActorInfo`) (`self.CombatTarget`) :!label _label)
      (`self.K2_EndAbility`))
    (:`OnInterrupted`
      (goto _label))
    (:`OnCancelled`
      (goto _label))))