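; GA_EnemyBlock is a gameplay ability, filed under Warrior enemy abilities, that puts an enemy into a blocking state.
; On activation it casts the avatar to BP_EnemyBase, binds EndBlocking to its block-finished delegate, sets the blocking flag by message and raises block chance to full.
; When the delegate fires, EndBlocking zeroes the block chance, clears the flag and ends the ability.
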(event `self.K2_ActivateAbility`
  (bind _asbp_enemy_base (cast `/Game/HorrorDungeon/Enemy/EnemyTypes/BP_EnemyBase` (`self.GetAvatarActorFromActorInfo`)))
  (bind _output_get (set `self.Enemy` _asbp_enemy_base))
  (add `BaseCharacter.BlockFinishedDelegate` _output_get (delegate `EndBlocking`))
  (message `CombatInterface.SetIsBlocking` (`self.GetAvatarActorFromActorInfo`) true)
  (`self.SetBlockChance` 100.0))

(event `EndBlocking`
  (`self.SetBlockChance` 0.0)
  (message `CombatInterface.SetIsBlocking` (`self.GetAvatarActorFromActorInfo`) false)
  (`self.K2_EndAbility`))