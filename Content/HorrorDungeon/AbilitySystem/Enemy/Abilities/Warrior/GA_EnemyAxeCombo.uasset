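; Gameplay ability for the Warrior enemy's axe attack: sets damage, turns toward the combat target and plays the montage tagged Attack.1.
; Gameplay events during the montage enable weapon collision at that montage's socket, clear the melee weapon's ignore list, and later disable collision.
; Montage completion, interruption or cancellation sends AttackEnd with the target and ends the ability.
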(event `self.K2_ActivateAbility`
  (`self.SetVariables`)
  (`self.SetDamage`)
  (bind _returnvalue (message `EnemyInterface.GetCombatTarget` (`self.GetAvatarActorFromActorInfo`)))
  (set `self.CombatTarget` _returnvalue)
  (message `CombatInterface.UpdateFacingTarget` (`self.GetAvatarActorFromActorInfo`) (`Actor.K2_GetActorLocation` (`self.CombatTarget`)))
  (bind _returnvalue_2 (message `CombatInterface.GetAbilityMontages` (`self.GetAvatarActorFromActorInfo`)))
  (bind (_montage _montagetag _sockettag) (break `TaggedMontage` (`self.GetTaggedMontage` _returnvalue_2 (struct :`TagName` "Montage.Attack.1"))))
  (`AbilityTask_PlayMontageAndWait.CreatePlayMontageAndWaitProxy` "None" _montage 1.0 "None" false
    (:`then`
      (`AbilityTask_WaitGameplayEvent.WaitGameplayEvent` (struct :`TagName` "Montage.Attack") null
        (:`then`
          (`AbilityTask_WaitGameplayEvent.WaitGameplayEvent` (struct :`TagName` "Montage.Attack.DisableCollision") null
            (:`EventReceived`
              (message `CombatInterface.DisableWeaponCollision` (`self.GetAvatarActorFromActorInfo`)))))
        (:`EventReceived`
          (message `CombatInterface.EnableWeaponCollision` (`self.GetAvatarActorFromActorInfo`) _sockettag)
          (`KismetArrayLibrary.Array_Clear` (`BaseWeapon.ActorsToIgnore` (`self.Melee Weapon`))))))
    (:`OnCompleted`
      (message `EnemyInterface.AttackEnd` (`self.GetAvatarActorFromActorInfo`) (`self.CombatTarget`) :!label _label)
      (`self.K2_EndAbility`))
    (:`OnInterrupted`
      (goto _label))
    (:`OnCancelled`
      (goto _label))))

(fn `SetVariables`
  (bind _asbp_enemy_base (cast `/Game/HorrorDungeon/Enemy/EnemyTypes/BP_EnemyBase` (`self.GetAvatarActorFromActorInfo`)))
  (bind _output_get (set `self.Enemy` _asbp_enemy_base))
  (bind _returnvalue (message `CombatInterface.GetEquippedWeapon1` _output_get))
  (bind _asbp_melee_weapon (cast `/Game/HorrorDungeon/Actor/Weapons/Melee/BP_MeleeWeapon` _returnvalue))
  (set `self.Melee Weapon` _asbp_melee_weapon))