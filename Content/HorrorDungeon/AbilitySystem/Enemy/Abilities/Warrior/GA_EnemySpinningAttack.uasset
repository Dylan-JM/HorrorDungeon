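; Gameplay ability for the sword enemy's spinning attack, which chases its combat target while the mesh spins.
; Caches the enemy and melee weapon, enlarges the weapon's ability hit box, sets damage, faces the target and plays a tagged attack montage.
; Parallel waits on montage gameplay events drive weapon collision handling and the spin chase.
; Montage completion, interruption or cancellation stops the spin, restores the box and ends the ability.
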(event `self.K2_ActivateAbility`
  (bind _enemysword (`self.EnemySword`))
  (bind _melee_weapon (`self.Melee Weapon`))
  (bind _abilityweaponbox (`MeleeWeapon.AbilityWeaponBox` (`self.Melee Weapon`)))
  (`self.SetVariables`)
  (`self.IncreaseWeaponAbilityBoxExtent`)
  (`self.SetDamage`)
  (bind _returnvalue (message `EnemyInterface.GetCombatTarget` (`self.GetAvatarActorFromActorInfo`)))
  (set `self.CombatTarget` _returnvalue)
  (message `CombatInterface.UpdateFacingTarget` (`self.GetAvatarActorFromActorInfo`) (`Actor.K2_GetActorLocation` (`self.CombatTarget`)))
  (bind _returnvalue_2 (message `CombatInterface.GetAbilityMontages` (`self.GetAvatarActorFromActorInfo`)))
  (`AbilityTask_PlayMontageAndWait.CreatePlayMontageAndWaitProxy` "None" (`.Montage` (break `TaggedMontage` (`self.GetTaggedMontage` _returnvalue_2 (struct :`TagName` "Montage.Attack.3")))) 1.0 "None" false
    (:`then`
      (`AbilityTask_WaitGameplayEvent.WaitGameplayEvent` (struct :`TagName` "Montage.Attack") null
        (:`then`
          (`AbilityTask_WaitGameplayEvent.WaitGameplayEvent` (struct :`TagName` "Montage.Attack.DisableCollision") null
            (:`then`
              (`AbilityTask_WaitGameplayEvent.WaitGameplayEvent` (struct :`TagName` "Montage.Attack.Spin") null
                (:`EventReceived`
                  (`/Game/HorrorDungeon/Enemy/EnemyTypes/BP_EnemySword.SpinMesh` _enemysword)
                  (`BaseEnemy.ChaseAttackTarget` _enemysword (`self.CombatTarget`)))))
            (:`EventReceived`
              (`MeleeWeapon.AbilityHandleCollision` (`self.Melee Weapon`) true))))
        (:`EventReceived`
          (`MeleeWeapon.AbilityHandleCollision` _melee_weapon true)
          (`KismetArrayLibrary.Array_Clear` (`MeleeWeapon.AbilityActorsToIgnore` _melee_weapon)))))
    (:`OnCompleted`
      (message `EnemyInterface.AttackEnd` (`self.GetAvatarActorFromActorInfo`) (`self.CombatTarget`) :!label _label)
      (`/Game/HorrorDungeon/Enemy/EnemyTypes/BP_EnemySword.StopSpinning` (`self.EnemySword`))
      (`BoxComponent.SetBoxExtent` _abilityweaponbox (/ (`BoxComponent.BoxExtent` _abilityweaponbox) (2.5 2.5 2.5)) true)
      (`self.K2_EndAbility`))
    (:`OnInterrupted`
      (goto _label))
    (:`OnCancelled`
      (goto _label))))

(fn `IncreaseWeaponAbilityBoxExtent`
  (bind _abilityweaponbox (`MeleeWeapon.AbilityWeaponBox` (`self.Melee Weapon`))
    (:`then`
      (`BoxComponent.SetBoxExtent` _abilityweaponbox (* (`BoxComponent.BoxExtent` _abilityweaponbox) (2.5 2.5 2.5)) true))
    (:`else`)))

(fn `SetVariables`
  (bind _asbp_enemy_sword (cast `/Game/HorrorDungeon/Enemy/EnemyTypes/BP_EnemySword` (`self.GetAvatarActorFromActorInfo`)))
  (bind _output_get (set `self.EnemySword` _asbp_enemy_sword))
  (bind _returnvalue (message `CombatInterface.GetEquippedWeapon1` _output_get))
  (bind _asbp_melee_weapon (cast `/Game/HorrorDungeon/Actor/Weapons/Melee/BP_MeleeWeapon` _returnvalue))
  (set `self.Melee Weapon` _asbp_melee_weapon))