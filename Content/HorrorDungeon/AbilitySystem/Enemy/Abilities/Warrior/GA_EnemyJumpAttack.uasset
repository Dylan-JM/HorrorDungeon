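; Gameplay ability for an enemy's jump attack, which leaps at its current combat target.
; It sets damage, updates facing toward the target and plays a tagged attack montage whose gameplay events trigger the jump and toggle weapon collision.
; The jump launches the character on a suggested projectile arc and stops movement on landing.
; When the montage completes or is interrupted or cancelled, it signals attack end and ends the ability.
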(event `self.K2_ActivateAbility`
  (bind _asbp_enemy_base (cast `/Game/HorrorDungeon/Enemy/EnemyTypes/BP_EnemyBase` (`self.GetAvatarActorFromActorInfo`)))
  (set `self.ControlledPawn` _asbp_enemy_base)
  (`self.SetDamage`)
  (bind _returnvalue (message `EnemyInterface.GetCombatTarget` (`self.GetAvatarActorFromActorInfo`)))
  (set `self.CombatTarget` _returnvalue)
  (message `CombatInterface.UpdateFacingTarget` (`self.GetAvatarActorFromActorInfo`) (`Actor.K2_GetActorLocation` (`self.CombatTarget`)))
  (bind _returnvalue_2 (message `CombatInterface.GetAbilityMontages` (`self.GetAvatarActorFromActorInfo`)))
  (bind (_montage _montagetag _sockettag) (break `TaggedMontage` (`self.GetTaggedMontage` _returnvalue_2 (struct :`TagName` "Montage.Attack.2"))))
  (`AbilityTask_PlayMontageAndWait.CreatePlayMontageAndWaitProxy` "None" _montage 1.0 "None" false
    (:`then`
      (`AbilityTask_WaitGameplayEvent.WaitGameplayEvent` (struct :`TagName` "Montage.Jump") null
        (:`then`
          (`AbilityTask_WaitGameplayEvent.WaitGameplayEvent` (struct :`TagName` "Montage.Attack") null
            (:`then`
              (`AbilityTask_WaitGameplayEvent.WaitGameplayEvent` (struct :`TagName` "Montage.Attack.DisableCollision") null
                (:`EventReceived`
                  (message `CombatInterface.DisableWeaponCollision` (`self.GetAvatarActorFromActorInfo`)))))
            (:`EventReceived`
              (message `CombatInterface.EnableWeaponCollision` (`self.GetAvatarActorFromActorInfo`) _sockettag))))
        (:`EventReceived`
          (`self.JumpToAttackTarget` (`self.CombatTarget`)))))
    (:`OnCompleted`
      (message `EnemyInterface.AttackEnd` (`self.GetAvatarActorFromActorInfo`) (`self.CombatTarget`) :!label _label)
      (`self.K2_EndAbility`))
    (:`OnInterrupted`
      (goto _label))
    (:`OnCancelled`
      (goto _label))))

(event `JumpToAttackTarget`
  (params (JumpTarget :type "Actor Object Reference"))
  (bind (_returnvalue_x _returnvalue_y) (`KismetMathLibrary.BreakVector` (`Actor.K2_GetActorLocation` JumpTarget)))
  (bind _controlledpawn (`self.ControlledPawn`))
  (bind _outlaunchvelocity (`GameplayStatics.SuggestProjectileVelocity_CustomArc` (`Actor.K2_GetActorLocation` _controlledpawn) (`KismetMathLibrary.MakeVector` _returnvalue_x _returnvalue_y (+ 0.0 100.0))))
  (`Character.LaunchCharacter` _controlledpawn _outlaunchvelocity true true)
  (add `Character.LandedDelegate` (`self.ControlledPawn`) (delegate `OnLandEvent`)))

(event `OnLandEvent`
  (params (Hit :type "HitResult Structure (by ref)"))
  (bind _controlledpawn (`self.ControlledPawn`))
  (remove `Character.LandedDelegate` _controlledpawn (delegate `OnLandEvent`))
  (`MovementComponent.StopMovementImmediately` (`Character.CharacterMovement` _controlledpawn)))