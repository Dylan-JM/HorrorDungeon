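; Zombie melee attack ability that sets damage, turns the avatar toward its combat target and plays a random montage matching the ability's tag.
; Montage gameplay events toggle weapon collision, with the socket tag taken from a repeated random montage lookup.
; When the montage completes, is interrupted or is cancelled, it notifies the avatar that the attack ended and ends the ability.
; Without a valid target, it ends immediately.
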(event `self.K2_ActivateAbility`
  (`self.SetDamage`)
  (bind _returnvalue (message `EnemyInterface.GetCombatTarget` (`self.GetAvatarActorFromActorInfo`)))
  (set `self.CombatTarget` _returnvalue)
  (bind _combattarget (`self.CombatTarget`)
    (:`then`
      (message `CombatInterface.UpdateFacingTarget` (`self.GetAvatarActorFromActorInfo`) (`Actor.K2_GetActorLocation` _combattarget))
      (bind _returnvalue_2 (message `CombatInterface.GetAbilityMontages` (`self.GetAvatarActorFromActorInfo`)))
      (bind (_montage _montagetag _sockettag) (break `TaggedMontage` (`self.GetRandomMontageWithTag` _returnvalue_2 (`|GetArrayItem` (`BlueprintGameplayTagLibrary.BreakGameplayTagContainer` (`self.GetAbilityTags`))))))
      (`AbilityTask_PlayMontageAndWait.CreatePlayMontageAndWaitProxy` "None" _montage 1.0 "None" false
        (:`then`
          (`AbilityTask_WaitGameplayEvent.WaitGameplayEvent` (struct :`TagName` "Montage.Attack") null
            (:`then`
              (`AbilityTask_WaitGameplayEvent.WaitGameplayEvent` (struct :`TagName` "Montage.Attack.DisableCollision") null
                (:`EventReceived`
                  (message `CombatInterface.DisableWeaponCollision` (`self.GetAvatarActorFromActorInfo`)))))
            (:`EventReceived`
              (message `CombatInterface.EnableWeaponCollision` (`self.GetAvatarActorFromActorInfo`) _sockettag))))
        (:`OnCompleted`
          (message `EnemyInterface.AttackEnd` (`self.GetAvatarActorFromActorInfo`) (`self.CombatTarget`) :!label _label)
          (`self.K2_EndAbility`))
        (:`OnInterrupted`
          (goto _label))
        (:`OnCancelled`
          (goto _label))))
    (:`else`
      (`self.K2_EndAbility`))))