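; Health potion pickup actor that also serves as an item for a grid-style inventory with dimensions and icons.
; When its owner overlaps it, it applies an instant Gameplay Effect to that owner and destroys itself.
; After a zero-length delay on BeginPlay, it fills its ItemObject with icon, class, size and type.
; GetDefaultItemObject constructs an equivalent BP_ItemObject through the GameInstance, using the same icon for both orientations.
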(event `self.ReceiveActorBeginOverlap`
  (params (OtherActor :type "Actor Object Reference"))
  (bind _returnvalue (`self.GetOwner`))
  (if (== OtherActor _returnvalue)
    (`self.ApplyEffectToTarget` _returnvalue (`self.InstantGameplayEffectClass`))
    (`self.K2_DestroyActor`)))

(event `self.ReceiveBeginPlay`
  (`KismetSystemLibrary.Delay` 0.0)
  (`self.SetItemObjectVariables`))

(event `self.SetItemObjectVariables`
  (set `ItemObject.ItemObjectValues` (make `ItemObjectValues` "/Game/HorrorDungeon/Actor/Weapons/Staff/M_IconHealthPotion.M_IconHealthPotion" "/Game/HorrorDungeon/Actor/Weapons/Staff/M_IconHealthPotion.M_IconHealthPotion" "BP_HealthPotion_C" (`self.Dimensions`) (`self.ItemType`)) (`self.ItemObject`)))

(fn `GetDefaultItemObject`
  (returns (ReturnValue :type "ItemObject Object Reference"))
  (bind _returnvalue (`|GenericCreateObject` (`GameplayStatics.GetGameInstance`) "/Game/HorrorDungeon/Actor/UObject/BP_ItemObject.BP_ItemObject_C" (make `ItemObjectValues` "/Game/HorrorDungeon/Actor/Weapons/Staff/M_IconHealthPotion.M_IconHealthPotion" "/Game/HorrorDungeon/Actor/Weapons/Staff/M_IconHealthPotion.M_IconHealthPotion" "BP_HealthPotion_C" (`self.Dimensions`) (`self.ItemType`)) false))
  (return _returnvalue))

(fn `UserConstructionScript`)