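; BP_ManaPotion is a mana potion item actor that also supplies its own item object data.
; When its owner overlaps it, it calls OnOverlap with that actor and destroys itself.
; After a zero-length delay on BeginPlay, it fills its ItemObject values with the potion icon, class, dimensions and item type.
; GetDefaultItemObject constructs a new BP_ItemObject through the game instance with matching icon, class, dimensions and type.
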(event `self.ReceiveActorBeginOverlap`
  (params (OtherActor :type "Actor Object Reference"))
  (if (== OtherActor (`self.GetOwner`))
    (`self.OnOverlap` OtherActor)
    (`self.K2_DestroyActor`)))

(event `self.ReceiveBeginPlay`
  (`KismetSystemLibrary.Delay` 0.0)
  (`self.SetItemObjectVariables`))

(event `self.SetItemObjectVariables`
  (set `ItemObject.ItemObjectValues` (make `ItemObjectValues` "/Game/HorrorDungeon/Actor/Weapons/Staff/M_IconManaPotion.M_IconManaPotion" "/Game/HorrorDungeon/Actor/Weapons/Staff/M_IconManaPotion.M_IconManaPotion" "BP_ManaPotion_C" (`self.Dimensions`) (`self.ItemType`)) (`self.ItemObject`)))

(fn `GetDefaultItemObject`
  (returns (ReturnValue :type "ItemObject Object Reference"))
  (bind _returnvalue (`|GenericCreateObject` (`GameplayStatics.GetGameInstance`) "/Game/HorrorDungeon/Actor/UObject/BP_ItemObject.BP_ItemObject_C" (make `ItemObjectValues` "/Game/HorrorDungeon/Actor/Weapons/Staff/M_IconManaPotion.M_IconManaPotion" "/Game/HorrorDungeon/Actor/Weapons/Staff/M_IconManaPotion.M_IconManaPotion" "BP_ManaPotion_C" (`self.Dimensions`) (`self.ItemType`)) false))
  (return _returnvalue))

(fn `UserConstructionScript`)