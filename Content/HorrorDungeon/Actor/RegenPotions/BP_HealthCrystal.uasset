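; BP_HealthCrystal is a health crystal consumable in the horror dungeon's regen potion set, with grid inventory item data.
; After a one-tick delay on BeginPlay, it fills its ItemObject with crystal icons, its own class, a square grid footprint and the Consumable type.
; When it overlaps its owning actor, it applies a duration gameplay effect to that owner and destroys itself.
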(event `self.ReceiveBeginPlay`
  (`KismetSystemLibrary.Delay` 0.0)
  (`self.SetItemObjectVariables`))

(event `self.ReceiveActorBeginOverlap`
  (params (OtherActor :type "Actor Object Reference"))
  (bind _returnvalue (`self.GetOwner`))
  (if (== OtherActor _returnvalue)
    (`self.ApplyEffectToTarget` _returnvalue (`self.DurationGameplayEffectClass`))
    (`self.K2_DestroyActor`)))

(event `self.SetItemObjectVariables`
  (bind _itemobject (`self.ItemObject`))
  (set `ItemObject.Icon` "/Game/HorrorDungeon/Actor/Weapons/Staff/M_IconCrystal.M_IconCrystal" _itemobject)
  (set `ItemObject.IconRotated` "/Game/HorrorDungeon/Actor/Weapons/Staff/M_IconCrystal.M_IconCrystal" _itemobject)
  (set `ItemObject.ItemClass` (`GameplayStatics.GetObjectClass` self) _itemobject)
  (set `ItemObject.Dimensions` (make `IntPoint` 2 2) _itemobject)
  (set `ItemObject.ItemType` "EIT_Consumable" _itemobject))

(fn `UserConstructionScript`)