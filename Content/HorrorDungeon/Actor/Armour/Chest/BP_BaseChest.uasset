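; BP_BaseChest is the chest armour item actor, supplying inventory data such as icons, grid dimensions and item type.
; After a zero-second Delay on BeginPlay, it fills its ItemObject with robe icon materials, its own class, Dimensions and ItemType.
; GetDefaultItemObject constructs and returns a BP_ItemObject with the same data, using the Game Instance as outer.
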(event `self.ReceiveBeginPlay`
  (`KismetSystemLibrary.Delay` 0.0)
  (`self.SetItemObjectVariables`))

(event `self.SetItemObjectVariables`
  (set `ItemObject.ItemObjectValues` (make `ItemObjectValues` "/Game/HorrorDungeon/Actor/Armour/Chest/PNGS/MI_Robes.MI_Robes" "/Game/HorrorDungeon/Actor/Armour/Chest/PNGS/MI_RobesRotated.MI_RobesRotated" "BP_BaseChest_C" (`self.Dimensions`) (`self.ItemType`)) (`self.ItemObject`)))

(fn `GetDefaultItemObject`
  (returns (ReturnValue :type "ItemObject Object Reference"))
  (bind _returnvalue (`|GenericCreateObject` (`GameplayStatics.GetGameInstance`) "/Game/HorrorDungeon/Actor/UObject/BP_ItemObject.BP_ItemObject_C" (make `ItemObjectValues` "/Game/HorrorDungeon/Actor/Armour/Chest/PNGS/MI_Robes.MI_Robes" "/Game/HorrorDungeon/Actor/Armour/Chest/PNGS/MI_RobesRotated.MI_RobesRotated" "BP_BaseChest_C" (`self.Dimensions`) (`self.ItemType`)) false))
  (return _returnvalue))

(fn `UserConstructionScript`)