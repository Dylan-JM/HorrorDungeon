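; BP_BaseLegs is the base leg armour item actor, supplying the data that represents it as an item object.
; On BeginPlay it waits on a zero-second Delay, then fills its ItemObject with normal and rotated icon materials, its class, dimensions and item type.
; GetDefaultItemObject constructs a new BP_ItemObject with the same values, using the game instance as outer.
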(event `self.ReceiveBeginPlay`
  (`KismetSystemLibrary.Delay` 0.0)
  (`self.SetItemObjectVariables`))

(event `self.SetItemObjectVariables`
  (set `ItemObject.ItemObjectValues` (make `ItemObjectValues` "/Game/HorrorDungeon/Actor/Armour/Legs/PNGS/MI_Legs.MI_Legs" "/Game/HorrorDungeon/Actor/Armour/Legs/PNGS/MI_LegsRotated.MI_LegsRotated" "BP_BaseLegs_C" (`self.Dimensions`) (`self.ItemType`)) (`self.ItemObject`)))

(fn `GetDefaultItemObject`
  (returns (ReturnValue :type "ItemObject Object Reference"))
  (bind _returnvalue (`|GenericCreateObject` (`GameplayStatics.GetGameInstance`) "/Game/HorrorDungeon/Actor/UObject/BP_ItemObject.BP_ItemObject_C" (make `ItemObjectValues` "/Game/HorrorDungeon/Actor/Armour/Legs/PNGS/MI_Legs.MI_Legs" "/Game/HorrorDungeon/Actor/Armour/Legs/PNGS/MI_LegsRotated.MI_LegsRotated" "BP_BaseLegs_C" (`self.Dimensions`) (`self.ItemType`)) false))
  (return _returnvalue))

(fn `UserConstructionScript`)