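; Melee weapon item actor that supplies claymore inventory data and can visually grow with a glowing gold effect.
; BeginPlay fills the ItemObject values and caches the mesh material, while GetDefaultItemObject constructs a fresh BP_ItemObject.
; The first Tick creates a gold dynamic material instance.
; MeshChange swaps materials and plays or reverses glow and size timelines, scaling only the mesh's Y and Z.
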(event `self.SetItemObjectVariables`
  (set `ItemObject.ItemObjectValues` (make `ItemObjectValues` "/Game/HorrorDungeon/Actor/Weapons/PNGS/M_IconClaymore.M_IconClaymore" "/Game/HorrorDungeon/Actor/Weapons/PNGS/M_IconStaffRotated.M_IconStaffRotated" "BP_MeleeWeapon_C" (`self.Dimensions`) (`self.ItemType`)) (`self.ItemObject`)))

(event `self.ReceiveBeginPlay`
  (`self.SetItemObjectVariables`)
  (set `self.DefaultMaterial` (`PrimitiveComponent.GetMaterial` (`self.ItemMesh`) 0)))

(event `self.ReceiveTick`
  (params (DeltaSeconds :type "Float (single-precision)"))
  (if (not (`self.MICreated`))
    (bind _returnvalue (`KismetMaterialLibrary.CreateDynamicMaterialInstance` "/Game/StarterContent/Materials/MI_GoldShiny.MI_GoldShiny"))
    (set `self.GoldMaterial` _returnvalue)
    (set `self.MICreated` true)))

(event `MeshChange`
  (params (IncreaseSize :type Boolean))
  (bind _itemmesh (`self.ItemMesh`))
  (bind _relativescale3d_x (`KismetMathLibrary.BreakVector` (`SceneComponent.RelativeScale3D` _itemmesh)))
  (if IncreaseSize
    (`|ExecutionSequence`
      (:`then_0`
        (`PrimitiveComponent.SetMaterial` (`self.ItemMesh`) 0 (`self.GoldMaterial`)))
      (:`then_1`
        (bind (_direction _scaletrack) (`Timeline|GlowChange` :!label _label)
          (:`Update`
            (`MaterialInstanceDynamic.SetScalarParameterValue` (`self.GoldMaterial`) "Glow" _scaletrack))))
      (:`then_2`
        (bind (_direction_2 _scaletrack_2) (`Timeline|SizeChange` :!label _label_2)
          (:`Update`
            (bind (_returnvalue_x _returnvalue_y _returnvalue_z) (`KismetMathLibrary.BreakVector` (`KismetMathLibrary.MakeVector` _scaletrack_2 _scaletrack_2 _scaletrack_2)))
            (`SceneComponent.SetRelativeScale3D` _itemmesh (`KismetMathLibrary.MakeVector` _relativescale3d_x _returnvalue_y _returnvalue_z))))))
    (else
      (`|ExecutionSequence`
        (:`then_0`
          (goto _label :!via `Reverse`))
        (:`then_1`
          (goto _label_2 :!via `Reverse`))
        (:`then_2`
          (`PrimitiveComponent.SetMaterial` (`self.ItemMesh`) 0 (`self.DefaultMaterial`)))))))

(fn `GetDefaultItemObject`
  (returns (ReturnValue :type "ItemObject Object Reference"))
  (bind _returnvalue (`|GenericCreateObject` (`GameplayStatics.GetGameInstance`) "/Game/HorrorDungeon/Actor/UObject/BP_ItemObject.BP_ItemObject_C" (make `ItemObjectValues` "/Game/HorrorDungeon/Actor/Weapons/PNGS/M_IconClaymore.M_IconClaymore" "/Game/HorrorDungeon/Actor/Weapons/PNGS/M_IconClaymoreRotated.M_IconClaymoreRotated" "BP_MeleeWeapon_C" (`self.Dimensions`) (`self.ItemType`)) false))
  (return _returnvalue))

(fn `UserConstructionScript`)