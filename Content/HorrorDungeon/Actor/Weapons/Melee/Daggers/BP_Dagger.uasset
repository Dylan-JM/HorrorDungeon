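; BP_Dagger is a dagger weapon actor that describes itself as an inventory item with icons, class, dimensions and item type.
; Shortly after BeginPlay, it writes these values into its ItemObject, using the same icon for normal and rotated slots.
; GetDefaultItemObject constructs and returns a new BP_ItemObject owned by the game instance, using the separate rotated icon.
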(event `self.ReceiveBeginPlay`
  (`KismetSystemLibrary.Delay` 0.2)
  (`self.SetItemObjectVariables`))

(event `self.SetItemObjectVariables`
  (set `ItemObject.ItemObjectValues` (make `ItemObjectValues` "/Game/HorrorDungeon/Actor/Weapons/PNGS/M_IconDagger.M_IconDagger" "/Game/HorrorDungeon/Actor/Weapons/PNGS/M_IconDagger.M_IconDagger" "BP_Dagger_C" (`self.Dimensions`) (`self.ItemType`)) (`self.ItemObject`)))

(fn `GetDefaultItemObject`
  (returns (ReturnValue :type "ItemObject Object Reference"))
  (bind _returnvalue (`|GenericCreateObject` (`GameplayStatics.GetGameInstance`) "/Game/HorrorDungeon/Actor/UObject/BP_ItemObject.BP_ItemObject_C" (make `ItemObjectValues` "/Game/HorrorDungeon/Actor/Weapons/PNGS/M_IconDagger.M_IconDagger" "/Game/HorrorDungeon/Actor/Weapons/PNGS/M_IconDaggerR.M_IconDaggerR" "BP_Dagger_C" (`self.Dimensions`) (`self.ItemType`)) false))
  (return _returnvalue))

(fn `UserConstructionScript`)