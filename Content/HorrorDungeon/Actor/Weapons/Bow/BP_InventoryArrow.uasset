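; BP_InventoryArrow is the arrow item in the bow weapon set, defining how arrows are represented as a stackable inventory item.
; After a zero-length delay on BeginPlay, it fills its ItemObject's values with arrow icons, class, dimensions, type and stack data.
; GetDefaultItemObject constructs and returns a new BP_ItemObject through the GameInstance, carrying the same arrow data, including the five-stack limit and current count.
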(event `self.ReceiveBeginPlay`
  (`KismetSystemLibrary.Delay` 0.0)
  (`self.SetItemObjectVariables`))

(event `self.SetItemObjectVariables`
  (set `ItemObject.ItemObjectValues` (make `ItemObjectValues` "/Game/HorrorDungeon/Actor/Weapons/PNGS/M_IconArrow.M_IconArrow" "/Game/HorrorDungeon/Actor/Weapons/PNGS/M_IconArrowR.M_IconArrowR" "BP_InventoryArrow_C" (`self.Dimensions`) (`self.ItemType`) false false 5 (`self.CurrentStacks`)) (`self.ItemObject`)))

(fn `GetDefaultItemObject`
  (returns (ReturnValue :type "ItemObject Object Reference"))
  (bind _returnvalue (`|GenericCreateObject` (`GameplayStatics.GetGameInstance`) "/Game/HorrorDungeon/Actor/UObject/BP_ItemObject.BP_ItemObject_C" (make `ItemObjectValues` "/Game/HorrorDungeon/Actor/Weapons/PNGS/M_IconArrow.M_IconArrow" "/Game/HorrorDungeon/Actor/Weapons/PNGS/M_IconArrowR.M_IconArrowR" "BP_InventoryArrow_C" (`self.Dimensions`) (`self.ItemType`) false false 5 (`self.CurrentStacks`)) false))
  (return _returnvalue))

(fn `UserConstructionScript`)