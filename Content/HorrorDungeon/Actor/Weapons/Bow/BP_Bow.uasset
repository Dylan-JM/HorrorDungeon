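; Bow weapon Blueprint for the dungeon game, registering as a two-handed inventory item with its own icons.
; On BeginPlay it fills its ItemObject values and snaps the arrow mesh to the bow's projectile_spawn socket; GetDefaultItemObject constructs a matching item object.
; A server-to-multicast event pair toggles the fire component.
; HasArrow is an empty stub, with its inventory arrow search left disconnected.
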(event `self.ReceiveBeginPlay`
  (`KismetSystemLibrary.Delay` 0.0)
  (`self.SetItemObjectVariables`)
  (`SceneComponent.K2_AttachToComponent` (`self.ArrowMesh`) (`self.BowMeshComponent`) "projectile_spawn" "SnapToTarget" "KeepRelative" "KeepRelative" true))

(event `self.SetItemObjectVariables`
  (set `ItemObject.ItemObjectValues` (make `ItemObjectValues` "/Game/HorrorDungeon/Actor/Weapons/PNGS/M_IconElvenBow.M_IconElvenBow" "/Game/HorrorDungeon/Actor/Weapons/PNGS/M_IconElvenBowR.M_IconElvenBowR" "BP_Bow_C" (`self.Dimensions`) (`self.ItemType`) false true) (`self.ItemObject`)))

(event `ServerActivateFire`
  (params (ActivateFire :type Boolean))
  (`self.MultiActivateFire` ActivateFire))

(event `MultiActivateFire`
  (params (ActivateFire :type Boolean))
  (if ActivateFire
    (`ActorComponent.Activate` (`self.FireComponent`) false)
    (else
      (`ActorComponent.Deactivate` (`self.FireComponent`)))))

(fn `GetDefaultItemObject`
  (returns (ReturnValue :type "ItemObject Object Reference"))
  (bind _returnvalue (`|GenericCreateObject` (`GameplayStatics.GetGameInstance`) "/Game/HorrorDungeon/Actor/UObject/BP_ItemObject.BP_ItemObject_C" (make `ItemObjectValues` "/Game/HorrorDungeon/Actor/Weapons/PNGS/M_IconElvenBow.M_IconElvenBow" "/Game/HorrorDungeon/Actor/Weapons/PNGS/M_IconElvenBowR.M_IconElvenBowR" "BP_Bow_C" (`self.Dimensions`) (`self.ItemType`) false true) false))
  (return _returnvalue))

(fn `HasArrow`
  (returns (ReturnValue :type Boolean)))

(fn `UserConstructionScript`)