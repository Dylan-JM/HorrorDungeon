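; Base enemy Blueprint for the horror dungeon game that stocks its inventory with its weapon and supports motion-warped facing.
; On BeginPlay, non-zombie enemies wait a tick, find a world actor of the Weapon1 class and add its default item object to BP_InventoryComponent2, storing success in HasItem.
; UpdateFacingTarget sets the FacingTarget warp location.
; Spawn-scale timeline, random-roll and combat-target facing logic are left unwired.
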(event `self.AddEquippedItemsToInventory`
  (if (not (`GameplayStatics.ObjectIsA` self "/Game/HorrorDungeon/Enemy/EnemyTypes/Zombie/BP_Zombie.BP_Zombie_C"))
    (bind _asbp_inventory_component_2 (cast `/Game/HorrorDungeon/Player/Components/BP_InventoryComponent2` (`self.InventoryComponent`)))
    (bind _weapon1 (`self.Weapon1`)
      (:`then`
        (`KismetSystemLibrary.Delay` 0.0)
        (bind _returnvalue (`GameplayStatics.GetActorOfClass` _weapon1))
        (bind _returnvalue_2 (`EquippableActor.GetDefaultItemObject` _returnvalue))
        (bind _asbp_item_object (cast `/Game/HorrorDungeon/Actor/UObject/BP_ItemObject` _returnvalue_2))
        (bind _added (`/Game/HorrorDungeon/Player/Components/BP_InventoryComponent2.TryAddItem` _asbp_inventory_component_2 _asbp_item_object))
        (set `self.bHasItem` _added))
      (:`else`))))

(event `self.ReceiveBeginPlay`
  (`self.AddEquippedItemsToInventory`))

(event `self.ReceiveTick`
  (params (DeltaSeconds :type "Float (single-precision)")))

(event `CombatInterface.UpdateFacingTarget`
  (params (Target :type "Vector Structure (by ref)"))
  (`MotionWarpingComponent.AddOrUpdateWarpTargetFromLocation` (`self.MotionWarping`) "FacingTarget" Target))

(fn `UserConstructionScript`)