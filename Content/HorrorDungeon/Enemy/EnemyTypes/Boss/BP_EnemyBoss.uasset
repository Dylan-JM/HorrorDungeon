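; BP_EnemyBoss is the boss enemy Blueprint for HorrorDungeon, extending a parent class with its own health bar, combat ranges and movement speed.
; On BeginPlay it creates a boss health bar widget bound to itself, assigns the overlay widget controller and adds it to the viewport.
; GetIdealRange returns fixed attack and defend radii.
; SetMovementSpeed switches on the movement state but returns the same slow speed for every state.
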(event `self.ReceiveBeginPlay`
  (`parent.ReceiveBeginPlay`)
  (bind _returnvalue (`|CreateWidget` "/Game/HorrorDungeon/Player/UI/ProgressBar/WBP_BossHealthBar.WBP_BossHealthBar_C" null self))
  (`/Engine/EditorBlueprintResources/StandardMacros.IsValid` _returnvalue
    (:`Is Valid`
      (`MainHUD.SetWidgetController` _returnvalue "/Game/HorrorDungeon/Player/UI/WidgetController/BP_OverlayWidgetController.BP_OverlayWidgetController")
      (`UserWidget.AddToViewport` _returnvalue 0))))

(fn `GetIdealRange`
  (returns (AttackRadius :type "Float (single-precision)") (DefendRadius :type "Float (single-precision)"))
  (return 250.0 450.0))

(fn `SetMovementSpeed`
  (params (MovementSpeed :type "EMovementSpeed Enum" :default "EIT_Idle"))
  (returns (ReturnValue :type "Float (single-precision)"))
  (locals (Speed :type "Float (single-precision)" :default 0.0))
  (switch `EMovementSpeed` MovementSpeed
    (:`EIT_Idle`
      _)
    (:`EIT_Walking`
      _)
    (:`EIT_Jogging`
      _)
    (:`EIT_Sprinting`
      _))
  (bind _output_get (set `local.Speed` 100.0))
  (return _output_get))

(fn `UserConstructionScript`
  (`parent.UserConstructionScript`))