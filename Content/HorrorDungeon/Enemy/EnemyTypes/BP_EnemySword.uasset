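; BP_EnemySword is a sword enemy type that can spin its mesh while chasing a target.
; SpinMesh drives a timeline that adds twelve full yaw turns to the rotation cached in the construction script, and StopSpinning restores it.
; ChaseAttackTarget re-issues AI MoveTo after each successful arrival, following a short delay, while IsAttacking holds.
; GetIdealRange supplies this type's attack and defend radii.
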(event `SpinMesh`
  (bind (_meshrotationbeforespin_roll _meshrotationbeforespin_pitch _meshrotationbeforespin_yaw) (`KismetMathLibrary.BreakRotator` (`self.MeshRotationBeforeSpin`)))
  (bind (_direction _zrotationalpha) (`Timeline|SpinMeshTimeline` :!via `PlayFromStart`)
    (:`Update`
      (`SceneComponent.K2_SetRelativeRotation` (`self.Mesh`) (`KismetMathLibrary.MakeRotator` _meshrotationbeforespin_roll _meshrotationbeforespin_pitch (`KismetMathLibrary.Lerp` _meshrotationbeforespin_yaw (+ _meshrotationbeforespin_yaw 4320.0) _zrotationalpha)) false false))))

(event `self.ChaseAttackTarget`
  (params (AttackTarget :type "Actor Object Reference"))
  (`|AIMoveTo` self (0.0 0.0 0.0) AttackTarget 200.0
    (:`OnSuccess`
      (`KismetSystemLibrary.Delay` 0.1)
      (if (`self.bIsAttacking`)
        (`self.ChaseAttackTarget` AttackTarget)))))

(event `StopSpinning`
  (`TimelineComponent.Stop` (`self.SpinMeshTimeline`))
  (`SceneComponent.K2_SetRelativeRotation` (`self.Mesh`) (`self.MeshRotationBeforeSpin`) false false))

(fn `GetIdealRange`
  (returns (AttackRadius :type "Float (single-precision)") (DefendRadius :type "Float (single-precision)"))
  (return 150.0 450.0))

(fn `UserConstructionScript`
  (`parent.UserConstructionScript`)
  (set `self.MeshRotationBeforeSpin` (`SceneComponent.RelativeRotation` (`self.Mesh`))))