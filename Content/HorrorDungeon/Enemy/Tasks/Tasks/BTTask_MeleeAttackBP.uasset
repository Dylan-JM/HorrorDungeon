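; Behavior tree task in which an AI enemy runs a melee attack on the blackboard attack target.
; It requests attack tokens through AttackStartMessage, failing if refused, then sprints unfocused to the blackboard attack radius and refocuses on the target.
; It triggers a Gameplay Ability by tag and finishes on the character's attack-finished delegate, or immediately if activation fails.
; A failed move or cast sends AttackEndMessage but still finishes as success.
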(event `self.ReceiveExecuteAI`
  (params (OwnerController :type "AIController Object Reference") (ControlledPawn :type "Pawn Object Reference"))
  (bind _controlled_pawn (`self.Controlled Pawn`))
  (bind _returnvalue (message `EnemyInterface.AttackStart` ControlledPawn (`BTFunctionLibrary.GetBlackboardValueAsActor` (`self.AttackTargetKey`)) (`self.Tokens Needed`)))
  (if _returnvalue
    (set `self.Owner Controller` OwnerController)
    (bind _output_get (set `self.Controlled Pawn` ControlledPawn))
    ;[1 1 1] BTT_SetMovementSpeed
    (bind _returnvalue_2 (message `EnemyInterface.SetMovementSpeed` _output_get "EIT_Sprinting"))
    (`KismetSystemLibrary.PrintString` (`KismetStringLibrary.Conv_DoubleToString` _returnvalue_2))
    ;[1 1 1] BTT_ClearFocus
    (set `Pawn.bUseControllerRotationYaw` false (`self.Controlled Pawn`))
    (`AIController.K2_ClearFocus` (`self.Owner Controller`))
    ;[1 1 1] BTT_MoveToIdealRange
    (`|AIMoveTo` (`self.Controlled Pawn`) (0.0 0.0 0.0) (`BTFunctionLibrary.GetBlackboardValueAsActor` (`self.AttackTargetKey`)) (`BTFunctionLibrary.GetBlackboardValueAsFloat` (`self.AttackRadiusKey`))
      (:`OnSuccess`
        ;[1 1 1] SetFocus
        (`AIController.K2_SetFocus` (`self.Owner Controller`) (`BTFunctionLibrary.GetBlackboardValueAsActor` (`self.AttackTargetKey`)))
        (set `Pawn.bUseControllerRotationYaw` true (`self.Controlled Pawn`))
        ;[1 0.1458 0.1557] BTT_Attack
        (bind _asbase_character (cast `BaseCharacter` (`self.Controlled Pawn`))
          (:`then`
            (add `BaseCharacter.AttackFinishedDelegate` _asbase_character (delegate `AttackFinished`))
            (message `EnemyInterface.SetCombatTarget` _controlled_pawn (`BTFunctionLibrary.GetBlackboardValueAsActor` (`self.AttackTargetKey`)))
            (bind _returnvalue_3 (`AbilitySystemComponent.TryActivateAbilitiesByTag` (`AbilitySystemBlueprintLibrary.GetAbilitySystemComponent` _controlled_pawn) (`self.GameplayTag`) true))
            (if (not _returnvalue_3)
              (`self.FinishExecute` true)))
          (:`CastFailed`
            (message `EnemyInterface.AttackEnd` (`self.Controlled Pawn`) (`BTFunctionLibrary.GetBlackboardValueAsActor` (`self.AttackTargetKey`)))
            (`self.FinishExecute` true))))
      (:`OnFail`
        (message `EnemyInterface.AttackEnd` (`self.Controlled Pawn`) (`BTFunctionLibrary.GetBlackboardValueAsActor` (`self.AttackTargetKey`)))
        (`self.FinishExecute` true)))
    (else
      (`self.FinishExecute` false))))

(event `AttackFinished`
  ;[1 0.1458 0.1557] BTT_Attack
  (`self.FinishExecute` true))