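; Behavior tree task that makes the mage enemy perform a heal through the Gameplay Ability System.
; It casts the controlled pawn to BP_EnemyBase and tries to activate an ability by the heal gameplay tag, failing if activation does not succeed.
; On success it binds to the enemy's heal-finished delegate, then unbinds and finishes successfully when that delegate fires.
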(event `self.ReceiveExecuteAI`
  (params (OwnerController :type "AIController Object Reference") (ControlledPawn :type "Pawn Object Reference"))
  (bind _asbp_enemy_base (cast `/Game/HorrorDungeon/Enemy/EnemyTypes/BP_EnemyBase` ControlledPawn))
  ;[0.9235 1 0] Heal
  (bind _output_get (set `self.Enemy` _asbp_enemy_base))
  (bind _returnvalue (`AbilitySystemComponent.TryActivateAbilitiesByTag` (`AbilitySystemBlueprintLibrary.GetAbilitySystemComponent` _output_get) (`self.HealGameplayTag`) true))
  (if _returnvalue
    (add `BaseCharacter.HealFinishedDelegate` (`self.Enemy`) (delegate `HealFinished`))
    (else
      (`self.FinishExecute` false))))

(event `HealFinished`
  ;[0.9235 1 0] Heal
  (remove `BaseCharacter.HealFinishedDelegate` (`self.Enemy`) (delegate `HealFinished`))
  (`self.FinishExecute` true))