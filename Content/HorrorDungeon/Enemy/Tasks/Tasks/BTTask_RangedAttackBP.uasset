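; Behavior tree task that runs an enemy's ranged attack against the blackboard attack target.
; It requests the attack with a token cost, then focuses the target, enables controller yaw rotation and sets the enemy's combat state.
; It activates a gameplay ability by tag and finishes when the enemy's attack-finished delegate fires.
; Refused requests and failed activations fail the task, while a failed enemy cast ends the attack but reports success.
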(event `self.ReceiveExecuteAI`
  (params (OwnerController :type "AIController Object Reference") (ControlledPawn :type "Pawn Object Reference"))
  (bind _controlled_pawn (`self.Controlled Pawn`))
  (bind _returnvalue (message `EnemyInterface.AttackStart` ControlledPawn (`BTFunctionLibrary.GetBlackboardValueAsActor` (`self.AttackTarget`)) (`self.TokensNeeded`)))
  (if _returnvalue
    (set `self.Owner Controller` OwnerController)
    (set `self.Controlled Pawn` ControlledPawn)
    ;[1 1 1] SetFocus
    (`AIController.K2_SetFocus` (`self.Owner Controller`) (`BTFunctionLibrary.GetBlackboardValueAsActor` (`self.AttackTarget`)))
    (set `Pawn.bUseControllerRotationYaw` true (`self.Controlled Pawn`))
    ;[1 1 1] BTT_SetInCombat
    (bind _asbp_enemy_base (cast `/Game/HorrorDungeon/Enemy/EnemyTypes/BP_EnemyBase` (`self.Controlled Pawn`))
      (:`then`
        (`BaseEnemy.SetInCombat` _asbp_enemy_base (`self.In Combat`))
        ;[1 0.09896 0.09896] BTT_Attack
        (add `BaseCharacter.AttackFinishedDelegate` _asbp_enemy_base (delegate `AttackFinished`))
        (message `EnemyInterface.SetCombatTarget` _controlled_pawn (`BTFunctionLibrary.GetBlackboardValueAsActor` (`self.AttackTarget`)))
        (bind _returnvalue_2 (`AbilitySystemComponent.TryActivateAbilitiesByTag` (`AbilitySystemBlueprintLibrary.GetAbilitySystemComponent` _controlled_pawn) (`self.GameplayTag`) true))
        (if (not _returnvalue_2)
          (message `EnemyInterface.AttackEnd` (`self.Controlled Pawn`) (`BTFunctionLibrary.GetBlackboardValueAsActor` (`self.AttackTarget`)))
          (`self.FinishExecute` false)))
      (:`CastFailed`
        (message `EnemyInterface.AttackEnd` (`self.Controlled Pawn`) (`BTFunctionLibrary.GetBlackboardValueAsActor` (`self.AttackTarget`)))
        (`self.FinishExecute` true)))
    (else
      (`self.FinishExecute` false))))

(event `AttackFinished`
  ;[1 0.09896 0.09896] BTT_Attack
  (`self.FinishExecute` true))